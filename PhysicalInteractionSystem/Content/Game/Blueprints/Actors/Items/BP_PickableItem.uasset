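; BP_PickableItem is an interactable item that can be carried by the player and dropped back into the world.
; PickUp attaches it to the player's grip, scaled to fit the item container with physics off; Drop traces from the camera to place it and restores scale and physics.
; For VR players, interaction tracks grabbed state and the holding motion controller.
; Interaction and detection events are sent to a database.
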(event EventStartDetection
  (params (Player :type BP%20Player%20Object%20Reference))
  (|CallParentFunction Player)
  (CallFunction|SendInteractEventtoDB "NewEnumerator26"))

(event EventStopDetection
  (params (Player :type BP%20Player%20Object%20Reference))
  (|CallParentFunction Player)
  (CallFunction|SendInteractEventtoDB "NewEnumerator27"))

(event EventInteractwith
  (params (Player :type BP%20Player%20Object%20Reference))
  ;[1 1 1] Interact
  (|CallParentFunction Player)
  (Utilities|FlowControl|Sequence
    (:then_0
      (CallFunction|SendInteractEventtoDB "NewEnumerator6"))
    (:then_1
      (Utilities|FlowControl|Sequence
        (:then_0
          (Utilities|Casting|CastToBP_Player_TFP Player))
        (:then_1
          (bind _asbp_player_vr (Utilities|Casting|CastToBP_Player_VR Player))
          (bind _motioncontroller (CallFunction|GetGrabberMotionController _asbp_player_vr))
          (Variables|Default|SetCurrent%20Motion%20Controller _motioncontroller)
          (Variables|Default|SetGrabbed true))))))

(event EventCancelInteract
  (params (Player :type BP%20Player%20Object%20Reference))
  ;[1 1 1] Interact
  (|CallParentFunction Player)
  (Utilities|FlowControl|Sequence
    (:then_0
      (CallFunction|SendInteractEventtoDB "NewEnumerator7"))
    (:then_1
      (Utilities|FlowControl|Sequence
        (:then_0
          (Utilities|Casting|CastToBP_Player_TFP Player))
        (:then_1
          (Utilities|Casting|CastToBP_Player_VR Player)
          (Variables|Default|SetCurrent%20Motion%20Controller 0)
          (Variables|Default|SetGrabbed false))))))

(event EventBeginPlay
  (|CallParentFunction)
  (Variables|ItemInfo|SetOriScale (Transformation|GetActorScale3D)))

(fn ConstructionScript
  (|CallParentFunction))

(fn PickUp
  (params (Player :type BP%20Player%20TFP%20Object%20Reference))
  (Transformation|AttachComponentToComponent (Variables|/Game/Game/Blueprints/Characters/Players/BP_Player_TFP.BP_Player_TFP_C|GetItemGrip Player) "None" "SnapToTarget" "SnapToTarget" "KeepRelative" true)
  (Transformation|SetActorScale3D (* (* (Variables|ItemInfo|GetOriScale) (/ (.SphereRadius (Collision|GetComponentBounds (Variables|/Game/Game/Blueprints/Characters/Players/BP_Player_TFP.BP_Player_TFP_C|GetItemContainer Player))) (.SphereRadius (Collision|GetComponentBounds (Variables|Default|GetStaticMesh))))) 0.8))
  (Physics|SetSimulatePhysics (Variables|Default|GetStaticMesh) false)
  (Collision|SetCollisionEnabled (Variables|Default|GetStaticMesh) "NoCollision")
  (Rendering|SetVisibility (Variables|/Game/Game/Blueprints/Characters/Players/BP_Player_TFP.BP_Player_TFP_C|GetItemContainer Player) true false))

(fn Drop
  (params (Player :type BP%20Player%20TFP%20Object%20Reference))
  (bind _returnvalue (Transformation|GetActorRotation))
  (bind (_startpoint _endpoint) (Default|LookHitPoint Player (Variables|/Game/Game/Blueprints/Characters/Players/BP_Player.BP_Player_C|GetFollowCamera Player) 2e+02))
  (bind _outhit (Collision|LineTraceByChannel _startpoint _endpoint "TraceTypeQuery1" false (Utilities|Array|MakeArray Player) "None"))
  (Transformation|SetActorRelativeRotation "0, 0, 0")
  (Transformation|DetachFromActor "KeepWorld" "KeepWorld" "KeepWorld")
  (if (.bblockinghit _outhit)
    (Transformation|SetActorLocation (.location _outhit) false false)
    (else
      (Transformation|SetActorLocation _endpoint false false)))
  (Transformation|SetActorRotation (Math|Rotator|MakeRotator (.roll _returnvalue) 0.0 (.yaw _returnvalue)))
  (Transformation|SetActorScale3D (Variables|ItemInfo|GetOriScale))
  (Physics|SetSimulatePhysics (Variables|Default|GetStaticMesh) true)
  (Collision|SetCollisionEnabled (Variables|Default|GetStaticMesh) "QueryAndPhysics")
  (Rendering|SetVisibility (Variables|/Game/Game/Blueprints/Characters/Players/BP_Player_TFP.BP_Player_TFP_C|GetItemContainer Player) false false))

(fn GetGrabberMotionController
  (params (PlayerVR :type BP%20Player%20VR%20Object%20Reference))
  (if (== (Variables|/Game/Game/Blueprints/Characters/Players/BP_Player_VR.BP_Player_VR_C|GetGrabbedItemL PlayerVR) self)
    (return (Variables|/Game/Game/Blueprints/Characters/Players/BP_Player_VR.BP_Player_VR_C|GetMotionControllerLeft PlayerVR))
    (elif (== (Variables|/Game/Game/Blueprints/Characters/Players/BP_Player_VR.BP_Player_VR_C|GetGrabbedItemR PlayerVR) self)
      (return (Variables|/Game/Game/Blueprints/Characters/Players/BP_Player_VR.BP_Player_VR_C|GetMotionControllerRight PlayerVR))
      (else
        (return 0)))))