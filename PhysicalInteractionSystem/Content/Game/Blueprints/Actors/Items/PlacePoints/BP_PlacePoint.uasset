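; BP_PlacePoint is a placement spot that accepts one pickable item type, starting hidden and inactive until activated.
; BeginPlay finds the item's data table row, sets it on four display meshes scaled by bounds, and spins RotatePivot.
; While active and empty, Tick polls capsule overlaps, binding matching items' interaction-completed event to snap them in place without collision.
; Leaving the sphere frees the point; dispatchers report placement changes, and activation toggles empty/used Niagara rings.
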(event OnComponentEndOverlap(SphereCollider)
  (params (OverlappedComponent :type Primitive%20Component%20Object%20Reference) (OtherActor :type Actor%20Object%20Reference) (OtherComp :type Primitive%20Component%20Object%20Reference) (OtherBodyIndex :type Integer))
  (if (== OtherActor (Variables|Default|GetTargetPlaceActor))
    (CallFunction|RemoveItemfromPlacePoint)
    (EventDispatchers|UnbindEventfromEDInteractionCompleted (Variables|Default|GetTargetPlaceActor) (delegate Custom|AddItemToPlacePoint))
    (EventDispatchers|UnbindEventfromEDInteractionStarted (Variables|Default|GetTargetPlaceActor) (delegate Custom|RemoveItemFromPlacePoint))
    (Variables|Default|SetTargetPlaceActor 0)
    (Variables|Default|SetActorPlaced false)))

(event Custom|AddItemToPlacePoint
  (Variables|Default|GetTargetPlaceActor
    (:then
      (if (not (Variables|Default|GetActorPlaced))
        (Variables|Default|SetPlacedActor (Variables|Default|GetTargetPlaceActor))
        (Collision|SetCollisionObjectType (Variables|/Game/Game/Blueprints/Actors/Items/BP_InteractItemParent.BP_InteractItemParent_C|GetStaticMesh (Variables|Default|GetPlacedActor)) "ECC_WorldStatic")
        (Transformation|SetActorLocationAndRotation (Variables|Default|GetPlacedActor) (Transformation|GetWorldLocation (Variables|Default|GetActorPosition)))
        (Collision|SetCollisionEnabled (Variables|/Game/Game/Blueprints/Actors/Items/BP_InteractItemParent.BP_InteractItemParent_C|GetStaticMesh (Variables|Default|GetPlacedActor)) "NoCollision")
        (Variables|Default|SetActorPlaced true)
        (Default|CallEDItemPlaced (Variables|Default|GetPlacedActor) self)))
    (:else)))

(event Custom|ActivatePoint
  (params (Activate :type Boolean))
  (bind _output_get (Variables|Default|SetPointActive Activate))
  (Rendering|SetActorHiddenInGame (not _output_get))
  (if (Variables|Default|GetActorPlaced)
    (Rendering|SetVisibility (Variables|Default|GetEmpty%20Area%20Ring%20Niagara%20System) false false)
    (Rendering|SetVisibility (Variables|Default|GetUsed%20Area%20Ring%20Niagara%20System) true false)
    (else
      (Rendering|SetVisibility (Variables|Default|GetEmpty%20Area%20Ring%20Niagara%20System) true false)
      (Rendering|SetVisibility (Variables|Default|GetUsed%20Area%20Ring%20Niagara%20System) false false))))

(event Custom|GetValidItemsForPlacing
  (if (and (not (Variables|Default|GetActorPlaced)) (Variables|Default|GetPointActive))
    (bind _hitactor (CallFunction|GetValidItemforPlacing))
    (Utilities|IsValid _hitactor
      (:Is%20Valid
        (bind _canuse (CallFunction|CanUseHere _hitactor))
        (if _canuse
          (bind _asbp_pickable_item (Utilities|Casting|CastToBP_PickableItem _hitactor))
          (bind _output_get (Variables|Default|SetTargetPlaceActor _asbp_pickable_item))
          (EventDispatchers|BindEventtoEDInteractionCompleted _output_get (delegate Custom|AddItemToPlacePoint))
          (else
            (Default|CallEDItemTriedtoPlace))))
      (:Is%20Not%20Valid
        (Variables|Default|SetTargetPlaceActor 0)))))

(event Custom|RemoveItemFromPlacePoint
  (if (Variables|Default|GetActorPlaced)
    (Variables|Default|SetActorPlaced false)
    (CallFunction|ActivatePoint true)
    (Default|CallEDItemRemoved (Variables|Default|GetTargetPlaceActor) self)))

(event EventBeginPlay
  (Development|SetHiddeninGame (Variables|Default|GetDefaultSceneRoot) true false)
  (CallFunction|GetItemDatafromDataTable)
  (Components|Movement|SetUpdatedComponent (Variables|Default|GetRotatingMovement) (Variables|Default|GetRotatePivot))
  (CallFunction|SetMeshandScale (Utilities|Array|MakeArray (Variables|Default|GetStaticMesh1) (Variables|Default|GetStaticMesh2) (Variables|Default|GetStaticMesh3) (Variables|Default|GetStaticMesh4)))
  (CallFunction|ActivatePoint false))

(event EventTick
  (params (DeltaSeconds :type Float%20%28single-precision%29))
  (CallFunction|GetValidItemsforPlacing))

(fn ConstructionScript)

(fn GetItemDatafromDataTable
  (bind _outrownames (DataTable|GetDataTableRowNames (Variables|Default|GetItem%20Data%20DataTable)))
  (bind _array_element (Utilities|Array|ForEachLoopwithBreak _outrownames :!label _label)
    (:LoopBody
      (bind _returnvalue (Utilities|GetDataTableRow (Variables|Default|GetItem%20Data%20DataTable) _array_element)
        (:then
          (if (Utilities|Enum|Equal(Enum) (.Type (Utilities|Struct|BreakF_ItemData _returnvalue)) (Variables|Default|GetItem%20Type))
            (Variables|Default|SetItem%20Data _returnvalue)
            (goto _label Break)))))))

(fn SetMeshandScale
  (params (Ori%20Meshes :type Array%20of%20Static%20Mesh%20Component%20Object%20References))
  (for _array_element Ori%20Meshes
    (Components|StaticMesh|SetStaticMesh _array_element (.mesh (Variables|Default|GetItem%20Data)))
    (Transformation|SetWorldScale3D _array_element "1.000000,1.000000,1.000000")
    (Transformation|SetWorldScale3D _array_element (* (Transformation|GetWorldScale _array_element) (* (/ 7.0 (.SphereRadius (Collision|GetComponentBounds _array_element))) 0.8)))))

(fn GetValidItemforPlacing
  (bind _item_data (Variables|Default|GetItem%20Data))
  (bind _capsulecollider (Variables|Default|GetCapsuleCollider))
  (bind _overlappingactors (Collision|GetOverlappingActors _capsulecollider (.class _item_data) :!class /Script/Engine.PrimitiveComponent))
  (if (Utilities|Array|IsNotEmpty _overlappingactors)
    (return (Utilities|Array|Get(acopy) _overlappingactors))
    (else
      (return 0))))

(fn CanUseHere
  (params (Actor :type Actor%20Object%20Reference))
  (return (== (Utilities|GetClass Actor) (.class (Variables|Default|GetItem%20Data)))))

(fn UseHere
  (params (ActorToUse :type BP%20Pickable%20Item%20Object%20Reference))
  (return false))