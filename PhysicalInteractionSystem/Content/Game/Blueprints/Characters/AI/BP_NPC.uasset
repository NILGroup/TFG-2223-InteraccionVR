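; NPC character that shows its name on a text component and can turn to face the player who interacts with it.
; On interaction, if CanLookPlayer is set, it stores a target rotation toward the player's mesh, keeping its own pitch.
; Tick eases the capsule toward that rotation with RInterpTo and stops once within a small tolerance.
; It also caches the game instance and exposes a walk-speed setter; CancelInteract is empty.
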(event Custom|SetName
  (Rendering|Components|TextRender|SetText (Variables|Default|GetNPCName) (Utilities|Text|ToText(String) (Variables|NPCInfo|GetName))))

(event Custom|CheckIfLookingAtPlayer
  ;[1 1 1] Look At Player
  (Variables|Player|SetLookPlayer (not (Math|Rotator|Equal(Rotator) (Transformation|GetWorldRotation (Variables|Collision|GetCapsuleComponent)) (Variables|Player|GetTargetRotation) 1e+01))))

(event Custom|LookAtPlayer
  (bind _player (Variables|Player|GetPlayer))
  (bind _capsulecomponent (Variables|Collision|GetCapsuleComponent))
  (bind _returnvalue (Transformation|GetWorldLocation _capsulecomponent))
  (bind _mesh (Variables|/Script/Engine.Character|GetMesh _player))
  (bind _returnvalue_2 (Transformation|GetWorldLocation _mesh))
  (bind _returnvalue_3 (Math|Rotator|FindLookatRotation _returnvalue _returnvalue_2))
  ;[1 1 1] Look At Player
  (Variables|Player|GetPlayer
    (:then
      (Variables|Player|SetTargetRotation (Math|Rotator|MakeRotator (.roll _returnvalue_3) (.pitch (Transformation|GetWorldRotation _capsulecomponent)) (.yaw _returnvalue_3)))
      (Variables|Player|SetLookPlayer true))
    (:else)))

(event EventBeginPlay
  (bind _asrr_game_instance (Utilities|Casting|CastToRR_GameInstance (Game|GetGameInstance)))
  (Variables|Default|SetGameInstance _asrr_game_instance)
  (CallFunction|SetName))

(event EventInteractwith
  (params (Player :type BP%20Player%20Object%20Reference))
  ;[1 1 1] Interact
  (Variables|Player|SetPlayer Player)
  (if (Variables|Player|GetCanLookPlayer)
    (CallFunction|LookatPlayer)))

(event EventCancelInteract
  (params (Player :type BP%20Player%20Object%20Reference))
  ;[1 1 1] Interact
)

(event EventTick
  (params (DeltaSeconds :type Float%20%28single-precision%29))
  (bind _capsulecomponent (Variables|Collision|GetCapsuleComponent))
  (Variables|Player|GetPlayer
    (:then
      (if (Variables|Player|GetLookPlayer)
        (if (Utilities|Enum|NotEqual(Enum) (Transformation|GetWorldRotation (Variables|Collision|GetCapsuleComponent)) (Variables|Player|GetTargetRotation))
          (Transformation|SetWorldRotation _capsulecomponent (Math|Interpolation|RInterpTo (Transformation|GetWorldRotation _capsulecomponent) (Variables|Player|GetTargetRotation) (Utilities|Time|GetWorldDeltaSeconds) 5.0) false false)
          (CallFunction|CheckifLookingatPlayer))))
    (:else)))

(fn ConstructionScript)

(fn UpdateWalkSpeed
  (params (Max%20Walk%20Speed :type Float%20%28double-precision%29))
  (Variables|/Script/Engine.CharacterMovementComponent|SetMaxWalkSpeed (Variables|Character|GetCharacterMovement) Max%20Walk%20Speed))