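; Base or child NPC Blueprint that the player can talk to by walking up and pressing an on-screen start-talking button.
; A talk-area overlap shows the button widget while no conversation runs; leaving hides it and stops the dialogue.
; Pressing the button triggers interaction, which forwards to the dialog manager component, wired to a typewriter text component.
; The dialog manager's conversation-finished event is relayed through the NPC's own dispatcher.
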(event OnComponentEndOverlap(TalkArea)
  (params (OverlappedComponent :type Primitive%20Component%20Object%20Reference) (OtherActor :type Actor%20Object%20Reference) (OtherComp :type Primitive%20Component%20Object%20Reference) (OtherBodyIndex :type Integer))
  ;[1 1 1] Talk Area
  (if (== OtherActor (Variables|Default|GetPlayer))
    (Default|StopConversation (Variables|Default|GetAC_DialogManager))
    (Development|SetHiddeninGame (Variables|Default|GetStartTalkingButtonWidgetComponent) true false)))

(event OnComponentBeginOverlap(TalkArea)
  (params (OverlappedComponent :type Primitive%20Component%20Object%20Reference) (OtherActor :type Actor%20Object%20Reference) (OtherComp :type Primitive%20Component%20Object%20Reference) (OtherBodyIndex :type Integer) (bFromSweep :type Boolean) (SweepResult :type Hit%20Result%20Structure%20%28by%20ref%29))
  ;[1 1 1] Talk Area
  (bind _asbp_player (Utilities|Casting|CastToBP_Player OtherActor))
  (if (and (Utilities|Array|IsNotEmpty (Collision|GetOverlappingActors (Variables|Default|GetTalkArea) "/Game/Game/Blueprints/Characters/Players/BP_Player.BP_Player_C" :!class /Script/Engine.PrimitiveComponent)) (not (Variables|/Game/Game/Blueprints/Components/AC_NPCDialogManager.AC_NPCDialogManager_C|GetIsTalking? (Variables|Default|GetAC_DialogManager))))
    (Variables|Default|SetPlayer _asbp_player)
    (Development|SetHiddeninGame (Variables|Default|GetStartTalkingButtonWidgetComponent) false false)))

(event Custom|NextConversation
  (Default|NextConversation (Variables|Default|GetAC_DialogManager)))

(event Custom|InitStartTalkingButton
  (Development|SetHiddeninGame (Variables|Default|GetDialogWidgetComponent) true false)
  (bind _aswbp_start_talking_button (Utilities|Casting|CastToWBP_StartTalkingButton (UserInterface|GetWidget (Variables|Default|GetStartTalkingButtonWidgetComponent))))
  (bind _output_get (Variables|Default|SetStartTalkingWidgetActor _aswbp_start_talking_button))
  (EventDispatchers|AssignEDStartTalking _output_get (delegate Custom|OnStartTalkingButtonPressed)))

(event Custom|OnStartTalkingButtonPressed
  (CallFunction|Interactwith (Variables|/Game/Game/Blueprints/RR_GameInstance.RR_GameInstance_C|GetCurrentPlayer (Variables|Default|GetGameInstance)))
  (Development|SetHiddeninGame (Variables|Default|GetStartTalkingButtonWidgetComponent) true false))

(event Custom|EventDispachedConversationFinished
  (params (Conversation%20Number :type Integer))
  (CallFunction|ConversationFinished Conversation%20Number))

(event Custom|Conversation%20Finished
  (params (Conversation%20Number :type Integer))
  (Default|CallEDConversationFinished Conversation%20Number))

(event EventBeginPlay
  (|CallParentFunction)
  (CallFunction|InitStartTalkingButton)
  (EventDispatchers|BindEventtoConversationFinished (Variables|Default|GetAC_DialogManager) (delegate Custom|EventDispachedConversationFinished))
  (Default|SetTypewriterComponent (Variables|Default|GetAC_DialogManager) (Variables|Default|GetAC_TypewriterText)))

(event EventInteractwith
  (params (Player :type BP%20Player%20Object%20Reference))
  ;[1 1 1] Interact
  (|CallParentFunction Player)
  (Default|Interactwith (Variables|Default|GetAC_DialogManager)))

(event EventCancelInteract
  (params (Player :type BP%20Player%20Object%20Reference))
  ;[1 1 1] Interact
  (|CallParentFunction Player))

(event EventTick
  (params (DeltaSeconds :type Float%20%28single-precision%29))
  (|CallParentFunction DeltaSeconds))

(fn ConstructionScript)