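; SenseGlove VR player pawn that visualizes fingertip touch as a debug aid for the finger colliders.
; BeginPlay gathers the five collider viewer meshes of each hand into left and right fingertip arrays.
; On touch updates while that hand is not grabbing, each fingertip swaps between real-hand and virtual-hand materials depending on whether it touches a valid actor.
; The grab-state handler checks for grabbing but takes no action.
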(event EventBeginPlay
  (Variables|Default|SetLeftFingertips (Utilities|Array|MakeArray (Variables|Default|GetThumbColliderViewer1) (Variables|Default|GetIndexColliderViewer1) (Variables|Default|GetMiddleColliderViewer1) (Variables|Default|GetRingColliderViewer1) (Variables|Default|GetPinkyColliderViewer1)))
  (Variables|Default|SetRightFingertips (Utilities|Array|MakeArray (Variables|Default|GetThumbColliderViewer) (Variables|Default|GetIndexColliderViewer) (Variables|Default|GetMiddleColliderViewer) (Variables|Default|GetRingColliderViewer) (Variables|Default|GetPinkyColliderViewer))))

(event Collision|EventActorBeginOverlap
  (params (OtherActor :type Actor%20Object%20Reference)))

(event EventTick
  (params (DeltaSeconds :type Float%20%28single-precision%29)))

(event EventOnGrabStateUpdated
  (params (GrabState :type SG%20Grab%20State%20Structure%20%28by%20ref%29))
  (if (Class|PawnKismetLibrary|IsGrabbing self (.Hand (Utilities|Struct|BreakSGGrabState GrabState)))
    _))

(event EventOnTouchStateUpdated
  (params (TouchState :type SG%20Touch%20State%20Structure%20%28by%20ref%29))
  (bind (_hand _actorthumbtouching _actorindextouching _actormiddletouching _actorringtouching _actorpinkytouching) (Utilities|Struct|BreakSGTouchState TouchState))
  ;[1 1 1] Debug de los colliders de las puntas de los dedos
  (if (not (Class|PawnKismetLibrary|IsGrabbing self _hand))
    (for (_array_element _array_index) (Utilities|Array|MakeArray _actorthumbtouching _actorindextouching _actormiddletouching _actorringtouching _actorpinkytouching)
      (Utilities|IsValid _array_element
        (:Is%20Valid
          (Rendering|Material|SetMaterial (select (Class|VirtualHandComponentKismetLibrary|IsRight _hand) (Utilities|Array|Get(acopy) (Variables|Default|GetRightFingertips) _array_index) (Utilities|Array|Get(acopy) (Variables|Default|GetLeftFingertips) _array_index)) 0 "/Game/SGTemplate/Materials/M_RealHand.M_RealHand"))
        (:Is%20Not%20Valid
          (Rendering|Material|SetMaterial (select (Class|VirtualHandComponentKismetLibrary|IsRight _hand) (Utilities|Array|Get(acopy) (Variables|Default|GetRightFingertips) _array_index) (Utilities|Array|Get(acopy) (Variables|Default|GetLeftFingertips) _array_index)) 0 "/Game/SGTemplate/Materials/M_VirtualHand.M_VirtualHand"))))))

(fn ConstructionScript)