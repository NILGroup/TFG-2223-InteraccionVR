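; Gameplay manager that tracks a scenario's steps and completion, registering itself with the GameInstance on BeginPlay.
; It loads steps from a DataTable, skipping the first row, shares them with the GameInstance and broadcasts changes to the current step.
; Step changes and completions are logged as timestamped database events.
; Ending gameplay saves tutorial data and closes the database, whose closed event triggers a delayed back-to-main-menu dispatcher.
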(event Custom|BindTuddyActions)

(event Custom|BindGameInstanceActions
  (EventDispatchers|AssignEDDatabaseClosed (Variables|Default|GetGameInstance) (delegate Custom|OnDatabaseClosed)))

(event Custom|BindNPCActions)

(event Custom|StartScenario)

(event Custom|AddItemToGameManagerImportantList
  (params (ItemType :type E_ItemType%20Enum :default "NewEnumerator2") (Actor :type Actor%20Object%20Reference)))

(event Custom|BindPlacePointsActions)

(event Custom|CompleteStep
  (params (GameplayStep :type E_GameplayStepTypes%20Enum :default "NewEnumerator0"))
  (CallFunction|SendGameplaySteptoDatabase GameplayStep "NewEnumerator3")
  (bind (_data _index) (CallFunction|GetStepDatabyType GameplayStep))
  (Utilities|Array|SetArrayElem (Variables|Steps|GetSteps) _index (Utilities|Struct|MakeF_GameplayStepData (.Type (Utilities|Struct|BreakF_GameplayStepData _data)) (.State (Utilities|Struct|BreakF_GameplayStepData _data)) (.Name (Utilities|Struct|BreakF_GameplayStepData _data)) (.Description (Utilities|Struct|BreakF_GameplayStepData _data)) true (.FinalScoreItem (Utilities|Struct|BreakF_GameplayStepData _data)) (.FinalScoreDescription (Utilities|Struct|BreakF_GameplayStepData _data))))
  (CallFunction|IsGameplayCompleted))

(event Custom|OnDatabaseClosed
  (Utilities|FlowControl|Delay 2.0)
  (Default|CallEDBacktoMainMenu))

(event Custom|OnGameInstancePlayerSetted
  (CallFunction|SetPlayerData))

(event Custom|EndGameplay
  (Default|SetGameplayStepsData (Variables|Default|GetGameInstance) (Variables|Steps|GetSteps))
  (Default|SaveData (Variables|Default|GetTutorialManager))
  (Default|CloseDatabase (Variables|Default|GetGameInstance)))

(event Custom|SetPlayerData
  (Variables|Default|SetPlayer (Variables|/Game/Game/Blueprints/RR_GameInstance.RR_GameInstance_C|GetCurrentPlayer (Variables|Default|GetGameInstance))))

(event Custom|BindPlayerActions)

(event Custom|SetCurrentGameplayStep
  (params (GameplayStepType :type E_GameplayStepTypes%20Enum :default "NewEnumerator9"))
  (bind _output_get (Variables|Steps|SetCurrentStepType GameplayStepType))
  (CallFunction|SetGameplayStepData _output_get)
  (Default|CallEDStepChanged (Variables|Steps|GetCurrentStepType))
  (CallFunction|SendGameplaySteptoDatabase (Variables|Steps|GetCurrentStepType) "NewEnumerator1"))

(event Custom|BindItemActions)

(event Custom|SetGameplayStepData
  (params (Step%20Type :type E_GameplayStepTypes%20Enum :default "NewEnumerator38"))
  (bind (_data _index) (CallFunction|GetStepDatabyType Step%20Type))
  (Variables|Steps|SetCurrentStepData _data)
  (Variables|Steps|SetCurrentStepIndex _index))

(event EventBeginPlay
  (Utilities|FlowControl|Sequence
    (:then_0
      (Variables|Default|SetGameplayCompleted false)
      (bind _asrr_game_instance (Utilities|Casting|CastToRR_GameInstance (Game|GetGameInstance)))
      (bind _output_get (Variables|Default|SetGameInstance _asrr_game_instance))
      (Variables|/Game/Game/Blueprints/RR_GameInstance.RR_GameInstance_C|SetGameplayManager _output_get self)
      (CallFunction|BindGameInstanceActions)
      (Variables|/Game/Game/Blueprints/RR_GameInstance.RR_GameInstance_C|GetCurrentPlayer _output_get
        (:then
          (CallFunction|SetPlayerData))
        (:else
          (EventDispatchers|BindEventtoEDPlayerSetted _output_get (delegate Custom|OnGameInstancePlayerSetted)))))
    (:then_1
      (CallFunction|GetStepsDatafromDataTable)
      (Default|SetGameplayStepsData (Variables|Default|GetGameInstance) (Variables|Steps|GetSteps)))
    (:then_2
      (if (Variables|Default|GetGameplayInOrder)
        (Default|CallEDOrderedGameplay)))))

(fn ConstructionScript)

(fn GetStepDatabyType
  (params (Step%20Type :type E_GameplayStepTypes%20Enum :default "NewEnumerator0"))
  (bind (_array_element _array_index) (Utilities|Array|ForEachLoopwithBreak (Variables|Steps|GetSteps) :!label _label)
    (:LoopBody
      (if (Utilities|Enum|Equal(Enum) (.Type (Utilities|Struct|BreakF_GameplayStepData _array_element)) Step%20Type)
        (goto _label Break)))
    (:Completed
      (return _array_element _array_index))))

(fn IsCurrentStep
  (params (Step :type E_GameplayStepTypes%20Enum :default "NewEnumerator0"))
  (return (Utilities|Enum|Equal(Enum) Step (Variables|Steps|GetCurrentStepType))))

(fn IsGameplayCompleted
  (bind _array_element (Utilities|Array|ForEachLoopwithBreak (Variables|Steps|GetSteps) :!label _label)
    (:LoopBody
      (if (.Completed (Utilities|Struct|BreakF_GameplayStepData _array_element))
        (Variables|Default|SetGameplayCompleted true)
        (else
          (Variables|Default|SetGameplayCompleted false)
          (goto _label Break))))))

(fn GetStepsDatafromDataTable
  (bind _outrownames (DataTable|GetDataTableRowNames (Variables|Default|GetSteps%20Data%20Table)))
  (Utilities|Array|RemoveIndex _outrownames)
  (for _array_element _outrownames
    (bind _returnvalue (Utilities|GetDataTableRow (Variables|Default|GetSteps%20Data%20Table) _array_element)
      (:then
        (Utilities|Array|Add (Variables|Steps|GetSteps) (Utilities|Struct|MakeF_GameplayStepData (.Type (Utilities|Struct|BreakF_GameplayStepData _returnvalue)) (.State (Utilities|Struct|BreakF_GameplayStepData _returnvalue)) (.Name (Utilities|Struct|BreakF_GameplayStepData _returnvalue)) (.Description (Utilities|Struct|BreakF_GameplayStepData _returnvalue)) (.Completed (Utilities|Struct|BreakF_GameplayStepData _returnvalue)) (.FinalScoreItem (Utilities|Struct|BreakF_GameplayStepData _returnvalue)) (.FinalScoreDescription (Utilities|Struct|BreakF_GameplayStepData _returnvalue))))))))

(fn SendGameplaySteptoDatabase
  (params (Step%20Type :type E_GameplayStepTypes%20Enum :default "NewEnumerator9") (Step%20State :type E_GameplayStepState%20Enum :default "NewEnumerator0"))
  (bind _data (Default|GetDataBaseMainInfoEvent (Variables|Default|GetGameInstance)))
  (bind _database_manager (Variables|/Game/Game/Blueprints/RR_GameInstance.RR_GameInstance_C|GetDatabase%20Manager (Variables|Default|GetGameInstance))
    (:then
      (Default|SendGameplayEventtoDB _database_manager (Utilities|Struct|MakeF_GameplayEvent 0 (.user_id (Utilities|Struct|BreakF_MainInfoEvent _data)) (.scenario_type (Utilities|Struct|BreakF_MainInfoEvent _data)) Step%20Type Step%20State (Math|DateTime|Now))))
    (:else
      (Default|Log (Variables|Default|GetGameInstance) "NewEnumerator2" "Falta el DatabaseManager en el GameInstance" false))))

(fn GetNextGameplayStepType
  (return (.type (Utilities|Array|Get(acopy) (Variables|Steps|GetSteps) (+ (Variables|Steps|GetCurrentStepIndex) 1)))))