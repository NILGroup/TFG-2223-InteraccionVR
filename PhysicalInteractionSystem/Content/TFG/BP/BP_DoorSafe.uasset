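; BP_DoorSafe is a child Blueprint, by its name a safe door, that relies on its parent class for behavior.
; BeginPlay, Released, Pickup and the construction script only forward to the parent implementations.
; ChangeState_1 branches on a Lock flag but performs no action and makes no parent call, while overlap and Tick are disabled stubs.
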(event Custom|ChangeState_1
  (params (Lock? :type Boolean))
  (if Lock?
    _))

(event EventBeginPlay
  (|CallParentFunction))

(event Collision|EventActorBeginOverlap
  (params (OtherActor :type Actor%20Object%20Reference))
  (|CallParentFunction OtherActor) ; This node is disabled and will not be called.\nDrag off pins to build functionality.
)

(event EventTick
  (params (DeltaSeconds :type Float%20%28single-precision%29))
  (|CallParentFunction DeltaSeconds) ; This node is disabled and will not be called.\nDrag off pins to build functionality.
)

(event EventReleased
  (|CallParentFunction))

(event EventPickup
  (params (Accurate :type Boolean) (Hit :type Hit%20Result%20Structure) (HideHandIco :type Boolean) (AttachTransform :type Motion%20Controller%20Component%20Object%20Reference))
  (|CallParentFunction Accurate Hit HideHandIco 0))

(fn ConstructionScript
  (|CallParentFunction))