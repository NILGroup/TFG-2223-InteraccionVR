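; A sliding door actor variant with a child handle actor, wired up at construction.
; The construction script casts the Handle2 child actor to BP_Handle, adds the door to that handle's connected actors and sets its attach target to the door's MainMesh.
; The event graph holds only disabled default events, so any sliding behavior lives outside this file.
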(event EventBeginPlay
  (|CallParentFunction) ; This node is disabled and will not be called.\nDrag off pins to build functionality.
)

(event Collision|EventActorBeginOverlap
  (params (OtherActor :type Actor%20Object%20Reference))
  (|CallParentFunction OtherActor) ; This node is disabled and will not be called.\nDrag off pins to build functionality.
)

(event EventTick
  (params (DeltaSeconds :type Float%20%28single-precision%29))
  (|CallParentFunction DeltaSeconds) ; This node is disabled and will not be called.\nDrag off pins to build functionality.
)

(fn ConstructionScript
  (bind _self self)
  (bind _handle2 (Variables|Default|GetHandle2))
  (bind _childactor (Variables|/Script/Engine.ChildActorComponent|GetChildActor _handle2))
  (bind _asbp_handle (Utilities|Casting|CastToBP_Handle _childactor))
  (|CallParentFunction)
  (Utilities|Array|Add (Variables|/Game/TFG/BP/BP_Handle.BP_Handle_C|GetConnectedActors _asbp_handle) _self)
  (Variables|/Game/TFG/BP/TFG_BP_BasePhysics.TFG_BP_BasePhysics_C|SetToAttach _asbp_handle (Utilities|Struct|Makes_ToAttach _self "MainMesh")) ; Connect the handle to the door
)