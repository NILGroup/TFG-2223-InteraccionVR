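; BP_w_Details is a debug actor that shows details about a connected actor on a w_Details widget.
; On BeginPlay it caches the widget component's user widget and fills two pairs of feature label and value texts from its variables.
; Every Tick it displays whether the connected actor's tick is enabled.
; DInteractFloat and DInteractBool events write incoming values to the widget's Value text.
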(event EventBeginPlay
  (bind _asw_details (Utilities|Casting|CastTow_Details (UserInterface|GetUserWidgetObject (Variables|Default|GetWidget))))
  (bind _output_get (Variables|Default|SetWDetails _asw_details))
  (Rendering|Components|TextRender|SetText (Variables|/Game/TFG/Widgets/Debug/w_Details.w_Details_C|GetAdditionalFeature _output_get) (Variables|Default|GetAdditionalFeature))
  (Rendering|Components|TextRender|SetText (Variables|/Game/TFG/Widgets/Debug/w_Details.w_Details_C|GetAdditionalFeatureValue _output_get) (Variables|Default|GetAdditionalFeatureValue))
  (Rendering|Components|TextRender|SetText (Variables|/Game/TFG/Widgets/Debug/w_Details.w_Details_C|GetAdditionalFeature_1 _output_get) (Variables|Default|GetAdditionalFeature1))
  (Rendering|Components|TextRender|SetText (Variables|/Game/TFG/Widgets/Debug/w_Details.w_Details_C|GetAdditionalFeatureValue_1 _output_get) (Variables|Default|GetAdditionalFeatureValue1)))

(event Collision|EventActorBeginOverlap
  (params (OtherActor :type Actor%20Object%20Reference)))

(event EventDInteractFloat
  (params (Value :type Float%20%28double-precision%29) (Source :type Integer))
  (Rendering|Components|TextRender|SetText (Variables|/Game/TFG/Widgets/Debug/w_Details.w_Details_C|GetValue (Variables|Default|GetWDetails)) (Utilities|Text|ToText(Float) Value "HalfToEven")))

(event EventTick
  (params (DeltaSeconds :type Float%20%28single-precision%29))
  (Rendering|Components|TextRender|SetText (Variables|/Game/TFG/Widgets/Debug/w_Details.w_Details_C|GetEventTick (Variables|Default|GetWDetails)) (Utilities|Text|ToText(Boolean) (Class|Actor|IsActorTickEnabled (Variables|Default|GetConnectedActor)))))

(event EventDInteractBool
  (params (Value :type Boolean) (Source :type Integer))
  (Rendering|Components|TextRender|SetText (Variables|/Game/TFG/Widgets/Debug/w_Details.w_Details_C|GetValue (Variables|Default|GetWDetails)) (Utilities|Text|ToText(Boolean) Value)))

(fn ConstructionScript)