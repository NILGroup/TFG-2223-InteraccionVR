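; VR door the player swings by grabbing either of two BP_HandlePoint child-actor knobs with a motion controller.
; While a knob is held, Tick yaws the mesh from the controller-to-door look-at angle, offset per knob and clamped around its starting rotation.
; If player opening is disallowed, knob events briefly show popup widgets ("Cerrado").
; AutomaticOpenAndLockDoor swings it open by timeline, without setting any lock flag.
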(event Custom|AutomaticOpenAndLockDoor
  (bind _orirotation (Variables|Default|GetOriRotation))
  (bind (_roll _pitch _yaw) (Math|Rotator|BreakRotator _orirotation))
  (Audio|Components|Audio|Play (Variables|Default|GetOpen) 0.0)
  (bind _newtrack_0 (Timeline|OpenDoorTimeline PlayFromStart)
    (:Update
      (Transformation|SetWorldRotation (Variables|Default|GetDoorMesh) (Math|Rotator|Lerp(Rotator) _orirotation (Math|Rotator|MakeRotator _roll _pitch (+ _yaw -9e+01)) _newtrack_0) false false))))

(event Custom|BindHandlePointActions
  (bind _asbp_handle_point (Utilities|Casting|CastToBP_HandlePoint (Variables|/Script/Engine.ChildActorComponent|GetChildActor (Variables|Default|GetKnob1))))
  (bind _output_get (Variables|Default|SetDoor%20Knob%201 _asbp_handle_point))
  (EventDispatchers|BindEventtoEDonKnobGrabStatusChanged _output_get (delegate Custom|OnKnobStatusChanged))
  (bind _asbp_handle_point_2 (Utilities|Casting|CastToBP_HandlePoint (Variables|/Script/Engine.ChildActorComponent|GetChildActor (Variables|Default|GetKnob2))))
  (bind _output_get_2 (Variables|Default|SetDoor%20Knob%202 _asbp_handle_point_2))
  (EventDispatchers|BindEventtoEDonKnobGrabStatusChanged _output_get_2 (delegate Custom|OnKnobStatusChanged)))

(event Custom|OnKnobStatusChanged
  (params (Grabbed :type Boolean))
  (if (Variables|Default|GetCanBeOpenedByPlayer)
    (bind _output_get (Variables|Default|SetKnob%20Grabbed Grabbed))
    (if _output_get
      (Audio|Components|Audio|Play (Variables|Default|GetOpen) 0.0))
    (else
      (CallFunction|ShowClosePopups))))

(event Custom|ShowClosePopups
  (Development|SetHiddeninGame (Variables|Default|GetWidget1) false false)
  (Development|SetHiddeninGame (Variables|Default|GetWidget2) false false)
  (Utilities|FlowControl|Delay 3.0)
  (Development|SetHiddeninGame (Variables|Default|GetWidget1) true false)
  (Development|SetHiddeninGame (Variables|Default|GetWidget2) true false))

(event EventBeginPlay
  (Variables|Default|SetOriRotation (Transformation|GetWorldRotation (Variables|Default|GetDoorMesh)))
  (bind _aswbp_popup_messages (Utilities|Casting|CastToWBP_PopupMessages (UserInterface|GetWidget (Variables|Default|GetWidget1))))
  (Default|SetPopupText _aswbp_popup_messages "Cerrado")
  (CallFunction|BindHandlePointActions))

(event EventTick
  (params (DeltaSeconds :type Float%20%28single-precision%29))
  (if (Variables|Default|GetKnob%20Grabbed)
    (bind _current_motion_controller (Variables|/Game/TFG/TFG_AleShit/Blueprints/Actors/Items/BP_PickableItem.BP_PickableItem_C|GetCurrent%20Motion%20Controller (Variables|Default|GetDoor%20Knob%201))
      (:then
        (CallFunction|SetDoorOpenAngle _current_motion_controller 85.0))
      (:else
        (bind _current_motion_controller_2 (Variables|/Game/TFG/TFG_AleShit/Blueprints/Actors/Items/BP_PickableItem.BP_PickableItem_C|GetCurrent%20Motion%20Controller (Variables|Default|GetDoor%20Knob%202))
          (:then
            (CallFunction|SetDoorOpenAngle _current_motion_controller_2 95.0))
          (:else))))))

(fn ConstructionScript)

(fn SetDoorOpenAngle
  (params (MotionController :type Motion%20Controller%20Component%20Object%20Reference) (AngleOffset :type Float%20%28double-precision%29))
  (bind _returnvalue (Transformation|GetWorldLocation MotionController))
  (bind _orirotation (Variables|Default|GetOriRotation))
  (bind _doormesh (Variables|Default|GetDoorMesh))
  (bind _returnvalue_2 (Transformation|GetWorldLocation _doormesh))
  (bind _returnvalue_3 (Math|Rotator|FindLookatRotation _returnvalue _returnvalue_2))
  (LocalVariables|SetCurrentAngleDifference (.yaw _returnvalue_3))
  (Transformation|SetWorldRotation (Variables|Default|GetDoorMesh) (Math|Rotator|MakeRotator 0.0 0.0 (Math|Float|ClampAngle (- (.yaw _returnvalue_3) AngleOffset) (- (.yaw _orirotation) 9e+01) (+ (.yaw _orirotation) 9e+01))) false false))