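; Tutorial variant of a pickable item that reports when the player first detects or grabs it, via event dispatchers.
; Spawn plays a pop sound, then after a short delay unhides the item, enables physics and makes it interactable; cancelling an interaction re-enables physics.
; A Liar flag overrides the grab type on BeginPlay, shows a widget on detection and suppresses the grab notification.
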(event Custom|Spawn
  (Audio|PlaySoundatLocation "/Game/TFG/TFG_AleShit/Assets/Sounds/effects/cartoon_pop.cartoon_pop" (Transformation|GetWorldLocation (Variables|Default|GetStaticMesh)) "0, 0, 0" 1.0 1.0 0.0 0 0 0 0)
  (Utilities|FlowControl|Delay 0.2)
  (Rendering|SetActorHiddenInGame false)
  (Physics|SetSimulatePhysics (Variables|Default|GetStaticMesh) true)
  (Variables|Default|SetCanBeInteracted true))

(event EventBeginPlay
  (|CallParentFunction)
  (if (Variables|Default|GetLiar)
    (Variables|/Game/VRTemplate/Blueprints/GrabComponent.GrabComponent_C|SetGrabType (Variables|Default|GetGrabComponent) "NewEnumerator0")))

(event EventCancelInteract
  (params (Player :type BP%20Player%20Object%20Reference))
  (|CallParentFunction Player)
  (Physics|SetSimulatePhysics (Variables|Default|GetStaticMesh) true))

(event EventStopDetection
  (params (Player :type BP%20Player%20Object%20Reference))
  (|CallParentFunction Player))

(event EventStartDetection
  (params (Player :type BP%20Player%20Object%20Reference))
  (|CallParentFunction Player)
  (if (Variables|Default|GetCanBeDetected)
    (Variables|Default|SetHasBeenDetected true)
    (Default|CallEDDetectionStarted)
    (if (Variables|Default|GetLiar)
      (Development|SetHiddeninGame (Variables|Default|GetWidget) false false))))

(event EventInteractwith
  (params (Player :type BP%20Player%20Object%20Reference))
  (|CallParentFunction Player)
  (if (and (not (Variables|Default|GetLiar)) (Variables|Default|GetCanBeGrabbed))
    (Variables|Default|SetHasBeenGrabbed true)
    (Default|CallEDInteractionStarted)))

(fn ConstructionScript
  (|CallParentFunction))