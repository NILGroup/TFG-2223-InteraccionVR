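; BP_RadiationEmissionPoint is an actor representing a radioactive isotope source that supplies dose rates and can contaminate actors.
; On BeginPlay it fills in the isotope's gamma constant from a DataTable.
; Dose functions apply inverse-square falloff with a minimum distance, converting curies and centimeters, plus exponential attenuation for shielding.
; When not encapsuled, mesh hits flag the other actor's AC_Radiation component as contaminated.
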(event OnComponentHit(StaticMesh)
  (params (HitComponent :type Primitive%20Component%20Object%20Reference) (OtherActor :type Actor%20Object%20Reference) (OtherComp :type Primitive%20Component%20Object%20Reference) (NormalImpulse :type Vector :default "0, 0, 0") (Hit :type Hit%20Result%20Structure%20%28by%20ref%29))
  (bind _returnvalue (Actor|GetComponentbyClass OtherActor "/Game/TFG/TFG_AleShit/Blueprints/Components/AC_Radiation.AC_Radiation_C"))
  (if (not (Variables|RadiationData|GetIsEncapsuled?))
    (Utilities|IsValid _returnvalue
      (:Is%20Valid
        (Variables|/Game/TFG/TFG_AleShit/Blueprints/Components/AC_Radiation.AC_Radiation_C|SetIsContamined? _returnvalue true)))))

(event Custom|SetIsotopeData
  (bind _isotopesdatatable (Variables|RadiationData|GetIsotopesDataTable))
  (bind _outrownames (DataTable|GetDataTableRowNames _isotopesdatatable))
  (bind _array_element (Utilities|Array|ForEachLoopwithBreak _outrownames :!label _label)
    (:LoopBody
      (bind _returnvalue (Utilities|GetDataTableRow _isotopesdatatable _array_element)
        (:then
          (if (Utilities|Enum|Equal(Enum) (.Isotope (Utilities|Struct|BreakF_IsotopesData _returnvalue)) (.Isotope (Utilities|Struct|BreakF_IsotopesData (Variables|RadiationData|GetIsotopeData))))
            (Variables|RadiationData|SetIsotopeData (Utilities|Struct|MakeF_IsotopesData (.Isotope (Utilities|Struct|BreakF_IsotopesData _returnvalue)) (.Gamma-rayConstant (Utilities|Struct|BreakF_IsotopesData _returnvalue))))
            (goto _label Break)))))))

(event EventBeginPlay
  (|CallParentFunction)
  (CallFunction|SetIsotopeData))

(event EventTick
  (params (DeltaSeconds :type Float%20%28single-precision%29))
  (|CallParentFunction DeltaSeconds))

(fn ConstructionScript)

(fn CalculateDoseRate
  (params (OtherActor :type Actor%20Object%20Reference))
  (bind _output_get (LocalVariables|SetDistance (Math|Vector|Distance(Vector) (Transformation|GetActorLocation OtherActor) (Transformation|GetActorLocation))))
  (if (< _output_get 1e+01)
    (LocalVariables|SetDistance 1e+01))
  (return (* (.Gamma-rayConstant (Utilities|Struct|BreakF_IsotopesData (Variables|RadiationData|GetIsotopeData))) (/ (* (Variables|RadiationData|GetActivity%20%28Ci%29) 37.0) (Math|Float|Square (/ (LocalVariables|GetDistance) 1e+02))))))

(fn CalculateShieldedDose
  (params (Other%20Actor :type Actor%20Object%20Reference) (Shielding%20Material%20Data :type F%20Shielding%20Material%20Data%20Structure) (Thickness :type Float%20%28double-precision%29))
  (bind _dose_rate (CallFunction|CalculateDoseRate Other%20Actor))
  (return (* _dose_rate (Class|KismetMathLibrary|Exp (* (/ (.AttenuationCoefficient (Utilities|Struct|BreakF_ShieldingMaterialData Shielding%20Material%20Data)) 1e+01) Thickness -1.0)))))