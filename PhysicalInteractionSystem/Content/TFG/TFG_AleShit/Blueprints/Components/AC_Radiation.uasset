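; Actor component that measures the radiation dose its owner receives from the level's BP_RadiationEmissionPoint.
; Each tick, while measuring is enabled, it asks the emitter for the dose rate, using the shielded calculation when the owner is inside an attenuation zone.
; It integrates the hourly rate over delta time into absorbed dose and tracks the peak rate.
; Events set zone shielding or reset absorption, and functions format readouts in mSv/h and mSv.
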(event Custom|CalculateRadiation
  (params (DeltaTime :type Float%20%28double-precision%29))
  ;[1 1 1] Calcula la tasa de radiación y la radiación absorbida en 1 segundo. Por eso cogemos DoseRate y la dividimos entre 3600 para que nos dé cuanta radiación absorvemos en 1 segundo
  (if (Variables|Default|GetCanMeasure?)
    (bind _radiactiveactor (Variables|Default|GetRadiactiveActor)
      (:then
        (if (Variables|Attenuation|GetInAttenuationZone)
          (bind _dose_rate (Default|CalculateShieldedDose _radiactiveactor (Variables|Default|GetOwner) (Variables|Attenuation|GetShieldingMaterialData) (Variables|Attenuation|GetShieldThickness)))
          (bind _output_get (Variables|Default|SetDoseRate _dose_rate))
          (Variables|Default|SetDoseAbsorption (+ (* (/ _output_get 3.6e+03) DeltaTime) (Variables|Default|GetDoseAbsorption)))
          (else
            (bind _dose_rate_2 (Default|CalculateDoseRate _radiactiveactor (Variables|Default|GetOwner)))
            (bind _output_get_2 (Variables|Default|SetDoseRate _dose_rate_2))
            (Variables|Default|SetDoseAbsorption (+ (* (/ _output_get_2 3.6e+03) DeltaTime) (Variables|Default|GetDoseAbsorption)))))
        (CallFunction|SetMaxDoseRate))
      (:else))))

(event Custom|EnterToAttenuationZone
  (params (Shield%20Data :type F%20Shielding%20Material%20Data%20Structure) (ShieldThickness :type Float%20%28double-precision%29))
  (Variables|Attenuation|SetInAttenuationZone true)
  (Variables|Attenuation|SetShieldingMaterialData Shield%20Data)
  (Variables|Attenuation|SetShieldThickness ShieldThickness))

(event Custom|ExitOfAttenuationZone
  (Variables|Attenuation|SetInAttenuationZone false)
  (Variables|Attenuation|SetShieldingMaterialData "")
  (Variables|Attenuation|SetShieldThickness 0.0))

(event Custom|RestartAbsorption
  (Variables|Default|SetDoseAbsorption 0.0))

(event Custom|SetMaxDoseRate
  (Variables|Default|SetMaxDoseRateReceived (Math|Float|Max(Float) (Variables|Default|GetDoseRate) (Variables|Default|GetMaxDoseRateReceived))))

(event EventBeginPlay
  (Variables|Default|SetOwner (Components|GetOwner))
  (bind _returnvalue (Actor|GetActorOfClass "/Game/TFG/TFG_AleShit/Blueprints/Actors/Radiation/BP_RadiationEmissionPoint.BP_RadiationEmissionPoint_C"))
  (Variables|Default|SetRadiactiveActor _returnvalue)
  (CallFunction|CalculateRadiation 0.0))

(event EventTick
  (params (DeltaSeconds :type Float%20%28single-precision%29))
  (CallFunction|CalculateRadiation DeltaSeconds))

(fn GetRateforDisplay
  (return (Utilities|Text|FormatText "{value} mSv/h" (Variables|Default|GetDoseRate))))

(fn GetAbsorptionforDisplay
  (return (Utilities|Text|FormatText "{value} mSv" (Variables|Default|GetDoseAbsorption))))