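; Database manager actor that forwards gameplay telemetry (users, interactions, radiation, movement, input and more) to a local-file database object.
; On the server it registers with RR_GameInstance, but its database spawn has no class and LocalFileDB is set to None.
; Send events create queries on that object when valid, and Tick flushes them on a timer.
; It relays closed and player-ID callbacks, and announces shutdown before a delayed close.
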(event Custom|OnPlayerIdFound
  (params (Id :type Integer))
  (Default|CallEDPlayerIdFound Id))

(event Custom|Get%20User%20Id
  (params (Player%20Name :type String))
  (bind _localfiledb (Variables|Default|GetLocalFileDB)
    (:then
      (Default|GetUserId _localfiledb Player%20Name))
    (:else)))

(event Custom|BindLocalFileDatabaseActions
  (bind _localfiledb (Variables|Default|GetLocalFileDB))
  (EventDispatchers|BindEventtoEDDatabaseClosed _localfiledb (delegate Custom|OnServerDatabaseClosed))
  (EventDispatchers|BindEventtoEDPlayerIdFound _localfiledb (delegate Custom|OnPlayerIdFound)))

(event Custom|StopAndCloseDatabase
  (Default|CallEDDatabaseNeedtobeClosed)
  (Utilities|FlowControl|Delay 1.0)
  (bind _localfiledb (Variables|Default|GetLocalFileDB)
    (:then
      (CallFunction|StopandCloseDatabase _localfiledb))
    (:else)))

(event Custom|OnServerDatabaseClosed
  (Variables|Default|SetLocalFileClosed false)
  (Default|CallEDDatabaseClosed))

(event EventBeginPlay
  (Networking|SwitchHasAuthority
    (:Authority
      (Utilities|FlowControl|Sequence
        (:then_0
          (bind _asrr_game_instance (Utilities|Casting|CastToRR_GameInstance (Game|GetGameInstance)))
          (bind _output_get (Variables|Default|SetGame%20Instance _asrr_game_instance))
          (Default|SetCurrentDataBase _output_get self))
        (:then_1
          (bind _returnvalue (Game|SpawnActorfromClass 0 (Math|Transform|MakeTransform "0, 0, 0") "Undefined" "OverrideRootScale" 0 0))
          (Variables|Default|SetLocalFileDB 0 _returnvalue)
          (CallFunction|BindLocalFileDatabaseActions))))))

(event EventTick
  (params (DeltaSeconds :type Float%20%28single-precision%29))
  (bind _output_get (Variables|Default|SetCurrentTimeToSendQuerys (+ DeltaSeconds (Variables|Default|GetCurrentTimeToSendQuerys))))
  (if (>= _output_get (Variables|Default|GetTimeToSendQuerys))
    (Variables|Default|SetCurrentTimeToSendQuerys 0.0)
    (bind _localfiledb (Variables|Default|GetLocalFileDB)
      (:then
        (Default|SendUpdateQuerystoDB _localfiledb))
      (:else))))

(event Custom|Send%20Item%20Interaction%20Event%20to%20DB
  (params (Data :type F%20Item%20Interaction%20Event%20Structure))
  (bind _localfiledb (Variables|Default|GetLocalFileDB)
    (:then
      (Default|CreateItemInteractionEventQuery _localfiledb Data))
    (:else)))

(event Custom|Send%20NPC%20Interaction%20Event%20to%20DB
  (params (Data :type F%20NPC%20Interaction%20Event%20Structure))
  (bind _localfiledb (Variables|Default|GetLocalFileDB)
    (:then
      (Default|CreateNPCInteractionEventQuery _localfiledb Data))
    (:else)))

(event Custom|Send%20RBQ%20Event%20To%20DB
  (params (Data :type F%20RBQ%20Event%20Structure))
  (bind _localfiledb (Variables|Default|GetLocalFileDB)
    (:then
      (Default|CreateRBQEventQuery _localfiledb Data))
    (:else)))

(event Custom|Send%20Item%20Radiation%20Event%20To%20DB
  (params (Data :type F%20Item%20Radiation%20Event%20Structure))
  (bind _localfiledb (Variables|Default|GetLocalFileDB)
    (:then
      (Default|CreateItemRadiationEventQuery _localfiledb Data))
    (:else)))

(event Custom|Send%20NPC%20Radiation%20Event%20To%20DB
  (params (Data :type F%20NPC%20Radiation%20Event%20Structure))
  (bind _localfiledb (Variables|Default|GetLocalFileDB)
    (:then
      (Default|CreateNPCRadiationEventQuery _localfiledb Data))
    (:else)))

(event Custom|Send%20EPD%20Radiation%20Event%20To%20DB
  (params (Data :type F%20EPD%20Radiation%20Event%20Structure))
  (bind _localfiledb (Variables|Default|GetLocalFileDB)
    (:then
      (Default|CreateEPDRadiationEventQuery _localfiledb Data))
    (:else)))

(event Custom|Send%20Help%20Panel%20Event%20To%20DB
  (params (Data :type F%20Help%20Panel%20Event%20Structure))
  (bind _localfiledb (Variables|Default|GetLocalFileDB)
    (:then
      (Default|CreateHelpPanelEventQuery _localfiledb Data))
    (:else)))

(event Custom|Send%20User%20Radiation%20Event%20To%20DB
  (params (Data :type F%20User%20Radiation%20Event%20Structure))
  (bind _localfiledb (Variables|Default|GetLocalFileDB)
    (:then
      (Default|CreateUserRadiationEventQuery _localfiledb Data))
    (:else)))

(event Custom|Send%20Tips%20Event%20To%20DB
  (params (Data :type F%20Tips%20Event%20Structure))
  (bind _localfiledb (Variables|Default|GetLocalFileDB)
    (:then
      (Default|CreateTipsEventQuery _localfiledb Data))
    (:else)))

(event Custom|SendClampsInteractionEventToDB
  (params (Data :type F%20Clamps%20Interaction%20Event%20Structure))
  (bind _localfiledb (Variables|Default|GetLocalFileDB)
    (:then
      (Default|CreateClampsInteractionEventQuery _localfiledb Data))
    (:else)))

(event Custom|SendInventoryEventToDB
  (params (Data :type F%20Inventory%20Event%20Structure))
  (bind _localfiledb (Variables|Default|GetLocalFileDB)
    (:then
      (Default|CreateInventoryEventQuery _localfiledb Data))
    (:else)))

(event Custom|SendUserInputEventToDB
  (params (Data :type F%20User%20Input%20Event%20Structure))
  (bind _localfiledb (Variables|Default|GetLocalFileDB)
    (:then
      (Default|CreateUserInputEventQuery _localfiledb Data))
    (:else)))

(event Custom|Send%20WalkieReport%20Event%20To%20DB
  (params (Data :type F%20Walkie%20Report%20Event%20Structure))
  (bind _localfiledb (Variables|Default|GetLocalFileDB)
    (:then
      (Default|CreateWalkieReportEventQuery _localfiledb Data))
    (:else)))

(event Custom|Send%20Move%20Event%20to%20DB
  (params (Data :type F%20Move%20Event%20Structure))
  (bind _localfiledb (Variables|Default|GetLocalFileDB)
    (:then
      (Default|CreateMoveEventQuery _localfiledb Data))
    (:else)))

(event Custom|Send%20Gameplay%20Event%20to%20DB
  (params (Data :type F%20Gameplay%20Event%20Structure))
  (bind _localfiledb (Variables|Default|GetLocalFileDB)
    (:then
      (Default|CreateGameplayEventQuery _localfiledb Data))
    (:else)))

(event Custom|Send%20User%20to%20DB
  (params (Data :type F%20User%20Structure))
  (bind _localfiledb (Variables|Default|GetLocalFileDB)
    (:then
      (Default|CreateUserQuery _localfiledb Data))
    (:else)))

(event Custom|Send%20PlacePoint%20Event%20to%20DB
  (params (Data :type F%20Place%20Point%20Event%20Structure))
  (bind _localfiledb (Variables|Default|GetLocalFileDB)
    (:then
      (Default|CreatePlacePointEventQuery _localfiledb Data))
    (:else)))

(fn ConstructionScript)