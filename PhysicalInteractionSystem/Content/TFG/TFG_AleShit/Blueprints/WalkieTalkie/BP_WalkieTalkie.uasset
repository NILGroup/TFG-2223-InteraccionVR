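; BP_WalkieTalkie is an interactable walkie-talkie, registered with the GameplayManager, through which the player makes initial and final reports via an in-world widget.
; Its ACWalkieDialogManager component handles interaction and runs conversations with a typewriter component, started by the widget's report buttons.
; When a conversation finishes, it hides the widget after a delay, fires that report's completion dispatcher and sets its flag.
; SetInitialConditions restores both flags and enables matching buttons; a completed final report blocks further interaction.
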(event Custom|BindEvents
  (bind _widgetactor (Variables|Default|GetWidgetActor))
  (EventDispatchers|BindEventtoEDInitialReportButtonClicked _widgetactor (delegate Custom|OnInitialReportButtonClicked))
  (EventDispatchers|BindEventtoEDFinalReportButtonClicked _widgetactor (delegate Custom|OnFinalReportButtonClicked))
  (EventDispatchers|BindEventtoConversationFinished (Variables|Default|GetAC_WalkieDialogManager) (delegate Custom|OnConversationFinished)))

(event Custom|OnConversationFinished
  (params (Walkie%20Conversation%20Type :type E_WalkieConversationType%20Enum :default "NewEnumerator0"))
  (Utilities|FlowControl|Delay 1.0)
  (Development|SetHiddeninGame (Variables|Default|GetWidgetComponent) true false)
  (switch Utilities|FlowControl|Switch|SwitchonE_WalkieConversationType Walkie%20Conversation%20Type
    (:NewEnumerator1
      (Default|CallEDInitialReportCompleted)
      (Variables|Default|SetInitialReportCompleted true))
    (:NewEnumerator2
      (Default|CallEDFinalReportCompleted)
      (Variables|Default|SetFinalReportCompleted true))))

(event Custom|SetInitialConditions
  (params (InitialReportCompleted :type Boolean) (FinalReportCompleted :type Boolean))
  (Variables|Default|SetInitialReportCompleted InitialReportCompleted)
  (Variables|Default|SetFinalReportCompleted FinalReportCompleted)
  (Default|EnableSpecificButtons (Variables|Default|GetWidgetActor) (not (Variables|Default|GetInitialReportCompleted)) (not (Variables|Default|GetFinalReportCompleted))))

(event Custom|OnFinalReportButtonClicked
  (Default|StartConversation (Variables|Default|GetAC_WalkieDialogManager) "NewEnumerator2"))

(event Custom|OnInitialReportButtonClicked
  (Default|StartConversation (Variables|Default|GetAC_WalkieDialogManager) "NewEnumerator1"))

(event EventBeginPlay
  (|CallParentFunction)
  (Utilities|FlowControl|Sequence
    (:then_0
      (bind _aswbp_walkie_talkie (Utilities|Casting|CastToWBP_WalkieTalkie (UserInterface|GetWidget (Variables|Default|GetWidgetComponent))))
      (bind _output_get (Variables|Default|SetWidgetActor _aswbp_walkie_talkie))
      (Default|SetOwner _output_get self)
      (Default|SetWidgetComponent (Variables|Default|GetAC_WalkieDialogManager) (Variables|Default|GetWidgetComponent) (Variables|Default|GetWidgetActor))
      (Default|SetTypewriterComponent (Variables|Default|GetAC_WalkieDialogManager) (Variables|Default|GetTypewriterText))
      (Development|SetHiddeninGame (Variables|Default|GetWidgetComponent) true false))
    (:then_1
      (bind _gameplaymanager (Variables|/Game/TFG/TFG_AleShit/Blueprints/RR_GameInstance.RR_GameInstance_C|GetGameplayManager (Variables|Default|GetGameInstance))
        (:then
          (Default|AddItemtoGameManagerImportantList _gameplaymanager (Variables|Default|GetItemType) self)
          (CallFunction|BindEvents))
        (:else)))))

(event EventCancelInteract
  (params (Player :type BP%20Player%20Object%20Reference))
  (|CallParentFunction Player)
  (Default|CancelInteract (Variables|Default|GetAC_WalkieDialogManager)))

(event EventInteractwith
  (params (Player :type BP%20Player%20Object%20Reference))
  (|CallParentFunction Player)
  (if (not (Variables|Default|GetFinalReportCompleted))
    (Default|Interactwith (Variables|Default|GetAC_WalkieDialogManager))))

(fn ConstructionScript
  (|CallParentFunction))