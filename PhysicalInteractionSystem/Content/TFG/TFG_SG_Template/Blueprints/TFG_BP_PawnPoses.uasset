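; VR glove pawn that handles two-handed grabbing and tests hand-pose recognition.
; On grab it hides the actor, changes its collision and spawns a pickup proxy at that hand's socket, tracked per hand.
; Release, also triggered by a disconnected glove on grab-state updates, copies proxy rotation back, restores collision and destroys the proxy.
; Tick compares the left hand against a thumbs-up pose, while number keys print joint data for debugging.
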(event EventOnGrabStateUpdated
  (params (GrabState :type SG%20Grab%20State%20Structure%20%28by%20ref%29))
  ;[1 1 1] DoubleHanded
  (if (not (Class|SGDeviceKismetLibrary|IsConnected (Class|VirtualHandComponentKismetLibrary|GetConnectedGlove (.Hand (Utilities|Struct|BreakSGGrabState GrabState)))))
    ;;[1 1 1] OnActorReleased
    (bind _output_get (Variables|Default|SetHand (stale EventOnActorReleased Hand)))
    (if (Class|VirtualHandComponentKismetLibrary|IsRight _output_get)
      (Variables|Default|SetGrabbedActor (Variables|Default|GetGrabbedActor_Right))
      (Variables|Default|SetSpawnedActor (Variables|Default|GetSpawnedActor_Right))
      (else
        (Variables|Default|SetGrabbedActor (Variables|Default|GetGrabbedActor_Left))
        (Variables|Default|SetSpawnedActor (Variables|Default|GetSpawnedActor_Left))))
    ;;;[1 1 1] Comprobar si es valida la llamada OnActorReleased
    (if (Utilities|IsValid (Variables|Default|GetSpawnedActor))
      (if (Utilities|IsValid (Variables|Default|GetGrabbedActor))
        (if (Utilities|IsValid (Variables|Default|GetHand))
          ;;;[1 1 1] Settear la rotacion de GrabbedActor con la de SpawnedActor y quitar la invisibilidad de GrabbedActor
          (Transformation|SetActorRotation (Variables|Default|GetGrabbedActor) (Transformation|GetWorldRotation (Variables|/Script/Engine.Actor|GetRootComponent (Variables|Default|GetSpawnedActor))) true)
          (Rendering|SetActorHiddenInGame (Variables|Default|GetGrabbedActor) false)
          ;;;[1 1 1] Activar Colision Objeto invisible y de la mano
          (for _array_element (Actor|GetComponentsByClass (Variables|Default|GetGrabbedActor) "/Script/Engine.StaticMeshComponent")
            (bind _asprimitive_component (Utilities|Casting|CastToPrimitiveComponent _array_element))
            (Collision|SetCollisionProfileName _asprimitive_component "BlockAll" true :!class /Script/Engine.PrimitiveComponent))
          (Collision|SetCollisionProfileName (Variables|Default|GetHand) "BlockAll" true :!class /Script/Engine.PrimitiveComponent)
          (Collision|SetCollisionObjectType (Variables|Default|GetHand) "ECC_Pawn")
          (Class|TFGSGIPickup|Drop(Message) (Variables|Default|GetSpawnedActor) false)
          ;;;[1 1 1] Eliminar las referencias de los objetos SpawnedActor y Grabbed Actor
          (Actor|DestroyActor (Variables|Default|GetSpawnedActor))
          (Variables|Default|SetSpawnedActor 0)
          (Variables|Default|SetGrabbedActor 0)
          (Variables|Default|SetLastGrabbedActor 0)
          (if (Class|VirtualHandComponentKismetLibrary|IsRight (Variables|Default|GetHand))
            (Variables|Default|SetGrabbedActor_Right 0)
            (Variables|Default|SetSpawnedActor_Right 0)
            (else
              (Variables|Default|SetGrabbedActor_Left 0)
              (Variables|Default|SetSpawnedActor_Left 0)))
          (Development|PrintString "Drop()" true true "(R=0.038153,G=1.000000,B=0.000000,A=1.000000)"))))))

(event Collision|EventActorBeginOverlap
  (params (OtherActor :type Actor%20Object%20Reference)))

(event EventOnActorGrabbed
  (params (Hand :type SG%20Virtual%20Hand%20Component%20Object%20Reference) (Actor :type Actor%20Object%20Reference))
  ;[1 1 1] DoubleHanded
  ;;[1 1 1] OnActorGrabbed
  ;;;[1 1 1] Diferenciar entre mano izquierda y derecha
  (bind _output_get (Variables|Default|SetHand Hand))
  (Variables|Default|SetGrabbedActor Actor)
  (if (Class|VirtualHandComponentKismetLibrary|IsRight _output_get)
    (Variables|Default|SetGrabbedActor_Right (Variables|Default|GetGrabbedActor))
    (else
      (Variables|Default|SetGrabbedActor_Left (Variables|Default|GetGrabbedActor))))
  ;;;[1 1 1] Comprobar si es valida la llamada OnActorGrabbed
  (if (not (== (Variables|Default|GetGrabbedActor) (Variables|Default|GetLastGrabbedActor)))
    (if (Utilities|IsValid (Variables|Default|GetGrabbedActor))
      (if (Utilities|IsValid (Variables|Default|GetHand))
        ;;;[1 1 1] Settear el Hit (posicion donde se atachea el objeto que vamos a spawnear)
        (if (Class|VirtualHandComponentKismetLibrary|IsRight (Variables|Default|GetHand))
          (Variables|Default|SetHit (Collision|MakeHitResult false false 0.0 0.0 "0, 0, 0" (Transformation|GetWorldLocation (Variables|Default|GetRightHandSocket)) "0,0,1" "0,0,1" 0 0))
          (else
            (Variables|Default|SetHit (Collision|MakeHitResult false false 0.0 0.0 "0, 0, 0" (Transformation|GetWorldLocation (Variables|Default|GetLeftHandSocket)) "0,0,1" "0,0,1" 0 0))))
        ;;;[1 1 1] Cambiar perfil de colisiones de Grabbed Actor (para que solo colisione con la mano) y hacerlo invisible
        (Variables|Default|SetLastGrabbedActor (Variables|Default|GetGrabbedActor))
        (for _array_element (Actor|GetComponentsByClass (Variables|Default|GetGrabbedActor) "/Script/Engine.StaticMeshComponent")
          (bind _asprimitive_component (Utilities|Casting|CastToPrimitiveComponent _array_element))
          (Collision|SetCollisionProfileName _asprimitive_component "TFG_GrabCollissions" true :!class /Script/Engine.PrimitiveComponent)
          ;;;[1 1 1] Settear SpawnedActor y cambiarle el perfil de colisiones para que no colisione con el GrabbedObject ni con la mano
          (bind _returnvalue (Game|SpawnActorfromClass "/Game/TFG/BP/TFG_SG_BP_PickUp.TFG_SG_BP_PickUp_C" (Transformation|GetActorTransform (Variables|Default|GetGrabbedActor)) "Undefined" "OverrideRootScale" 0 0))
          (Variables|Default|SetSpawnedActor _returnvalue)
          (if (Class|VirtualHandComponentKismetLibrary|IsRight (Variables|Default|GetHand))
            (Variables|Default|SetSpawnedActor_Right (Variables|Default|GetSpawnedActor))
            (else
              (Variables|Default|SetSpawnedActor_Left (Variables|Default|GetSpawnedActor))))
          (for _array_element_2 (Actor|GetComponentsByClass (Variables|Default|GetSpawnedActor) "/Script/Engine.StaticMeshComponent")
            (bind _asprimitive_component_2 (Utilities|Casting|CastToPrimitiveComponent _array_element_2))
            (Collision|SetCollisionProfileName _asprimitive_component_2 "TFG_SpawnPhysics" true :!class /Script/Engine.PrimitiveComponent)
            (Class|TFGSGIPickup|Pickup(Message) (Variables|Default|GetSpawnedActor) false (Variables|Default|GetHit) false (Variables|Default|GetHand))
            (Development|PrintString "Pickup()")))
        (Rendering|SetActorHiddenInGame (Variables|Default|GetGrabbedActor) true)))))

(event EventOnActorReleased
  (params (Hand :type SG%20Virtual%20Hand%20Component%20Object%20Reference) (Actor :type Actor%20Object%20Reference))
  ;[1 1 1] DoubleHanded
  ;;[1 1 1] OnActorReleased
  (bind _output_get (Variables|Default|SetHand Hand))
  (if (Class|VirtualHandComponentKismetLibrary|IsRight _output_get)
    (Variables|Default|SetGrabbedActor (Variables|Default|GetGrabbedActor_Right))
    (Variables|Default|SetSpawnedActor (Variables|Default|GetSpawnedActor_Right))
    (else
      (Variables|Default|SetGrabbedActor (Variables|Default|GetGrabbedActor_Left))
      (Variables|Default|SetSpawnedActor (Variables|Default|GetSpawnedActor_Left))))
  ;;;[1 1 1] Comprobar si es valida la llamada OnActorReleased
  (if (Utilities|IsValid (Variables|Default|GetSpawnedActor))
    (if (Utilities|IsValid (Variables|Default|GetGrabbedActor))
      (if (Utilities|IsValid (Variables|Default|GetHand))
        ;;;[1 1 1] Settear la rotacion de GrabbedActor con la de SpawnedActor y quitar la invisibilidad de GrabbedActor
        (Transformation|SetActorRotation (Variables|Default|GetGrabbedActor) (Transformation|GetWorldRotation (Variables|/Script/Engine.Actor|GetRootComponent (Variables|Default|GetSpawnedActor))) true)
        (Rendering|SetActorHiddenInGame (Variables|Default|GetGrabbedActor) false)
        ;;;[1 1 1] Activar Colision Objeto invisible y de la mano
        (for _array_element (Actor|GetComponentsByClass (Variables|Default|GetGrabbedActor) "/Script/Engine.StaticMeshComponent")
          (bind _asprimitive_component (Utilities|Casting|CastToPrimitiveComponent _array_element))
          (Collision|SetCollisionProfileName _asprimitive_component "BlockAll" true :!class /Script/Engine.PrimitiveComponent))
        (Collision|SetCollisionProfileName (Variables|Default|GetHand) "BlockAll" true :!class /Script/Engine.PrimitiveComponent)
        (Collision|SetCollisionObjectType (Variables|Default|GetHand) "ECC_Pawn")
        (Class|TFGSGIPickup|Drop(Message) (Variables|Default|GetSpawnedActor) false)
        ;;;[1 1 1] Eliminar las referencias de los objetos SpawnedActor y Grabbed Actor
        (Actor|DestroyActor (Variables|Default|GetSpawnedActor))
        (Variables|Default|SetSpawnedActor 0)
        (Variables|Default|SetGrabbedActor 0)
        (Variables|Default|SetLastGrabbedActor 0)
        (if (Class|VirtualHandComponentKismetLibrary|IsRight (Variables|Default|GetHand))
          (Variables|Default|SetGrabbedActor_Right 0)
          (Variables|Default|SetSpawnedActor_Right 0)
          (else
            (Variables|Default|SetGrabbedActor_Left 0)
            (Variables|Default|SetSpawnedActor_Left 0)))
        (Development|PrintString "Drop()" true true "(R=0.038153,G=1.000000,B=0.000000,A=1.000000)")))))

(event EventTick
  (params (DeltaSeconds :type Float%20%28single-precision%29))
  (bind _returnvalue (Class|VirtualHandComponentKismetLibrary|GetHandPose (Class|PawnKismetLibrary|GetHandLeft self)))
  (bind _returnvalue_2 (Class|SGHandPoseKismetLibrary|ThumbsUpBRH false))
  (if (Class|SGHandPoseKismetLibrary|Equals _returnvalue _returnvalue_2)
    (Development|PrintString "Puño")))

(event Input|KeyboardEvents|1
  (params (Key :type Key%20Structure :default "None"))
  (:Pressed
    (bind _returnvalue (Class|VirtualHandComponentKismetLibrary|GetHandPose (Class|PawnKismetLibrary|GetRealHandLeft self)))
    (for (_array_element _array_index) (Class|SGHandPoseKismetLibrary|GetJointPositions _returnvalue)
      (Development|PrintString (Utilities|String|ToString(Integer) _array_index) true true "(R=1.000000,G=0.000000,B=0.938498,A=1.000000)" 2e+01)
      (for _array_element_2 (Utilities|Struct|BreakSGVectorArray _array_element)
        (Development|PrintString (Utilities|String|ToString(Vector) _array_element_2) true true "(R=0.950594,G=0.000000,B=1.000000,A=1.000000)" 2e+01)))))

(event Input|KeyboardEvents|3
  (params (Key :type Key%20Structure :default "None"))
  (:Pressed
    (bind _returnvalue (Class|SGHandPoseKismetLibrary|FistBRH false))
    (for _array_element (Class|SGHandPoseKismetLibrary|GetJointPositions _returnvalue)
      (for _array_element_2 (Utilities|Struct|BreakSGVectorArray _array_element)
        (Development|PrintString (Utilities|String|ToString(Vector) _array_element_2) true true "(R=0.000000,G=1.000000,B=0.756028,A=1.000000)" 2e+01)))))

(event Input|KeyboardEvents|2
  (params (Key :type Key%20Structure :default "None"))
  (:Pressed
    (bind _returnvalue (Class|VirtualHandComponentKismetLibrary|GetHandPose (Class|PawnKismetLibrary|GetRealHandLeft self)))
    (for _array_element (Class|SGHandPoseKismetLibrary|GetJointRotations _returnvalue)
      (for _array_element_2 (Utilities|Struct|BreakSGRotatorArray _array_element)
        (Development|PrintString (Utilities|String|ToString(Rotator) _array_element_2) true true "(R=0.950594,G=0.000000,B=1.000000,A=1.000000)" 2e+01)))))

(event Input|KeyboardEvents|4
  (params (Key :type Key%20Structure :default "None"))
  (:Pressed
    (bind _returnvalue (Class|SGHandPoseKismetLibrary|FistBRH false))
    (for _array_element (Class|SGHandPoseKismetLibrary|GetJointRotations _returnvalue)
      (for _array_element_2 (Utilities|Struct|BreakSGRotatorArray _array_element)
        (Development|PrintString (Utilities|String|ToString(Rotator) _array_element_2) true true "(R=0.915912,G=1.000000,B=0.000000,A=1.000000)" 2e+01)))))

(fn ConstructionScript)