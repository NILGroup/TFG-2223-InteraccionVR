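; SenseGlove (SG) template pawn that handles hand grab and release through a stand-in pickup actor.
; On grab, it changes the grabbed actor's mesh collision, hides it and spawns a TFG_SG_BP_PickUp at its transform, attached via PickupMessage using the hand socket.
; On release, it drops and destroys the stand-in, copies only its rotation to the original, unhides it and restores object and hand collision.
; Debug prints and several disconnected test chains remain.
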(event EventBeginPlay)

(event Collision|EventActorBeginOverlap
  (params (OtherActor :type Actor%20Object%20Reference)))

(event EventTick
  (params (DeltaSeconds :type Float%20%28single-precision%29)))

(event EventOnActorGrabbed
  (params (Hand :type SG%20Virtual%20Hand%20Component%20Object%20Reference) (Actor :type Actor%20Object%20Reference))
  (Variables|Default|SetHand Hand)
  (Variables|Default|SetGrabbedActor Actor)
  ;[1 1 1] Quitar colision de la mano y del objeto invisible
  (if (Utilities|IsValid (Variables|Default|GetGrabbedActor))
    (for _array_element (Actor|GetComponentsByClass (Variables|Default|GetGrabbedActor) "/Script/Engine.StaticMeshComponent")
      (bind _asprimitive_component (Utilities|Casting|CastToPrimitiveComponent _array_element))
      (Collision|SetCollisionProfileName _asprimitive_component "TFG_GrabCollissions" true :!class /Script/Engine.PrimitiveComponent))
    (Rendering|SetActorHiddenInGame (Variables|Default|GetGrabbedActor) true)
    ;[1 1 1] Spawnear y Attachear Grabbed Actor a la mano
    (bind _returnvalue (Game|SpawnActorfromClass "/Game/TFG/BP/TFG_SG_BP_PickUp.TFG_SG_BP_PickUp_C" (Transformation|GetActorTransform (Variables|Default|GetGrabbedActor)) "Undefined" "OverrideRootScale" 0 0))
    (bind _output_get (Variables|Default|SetSpawnedActor _returnvalue))
    (for _array_element_2 (Actor|GetComponentsByClass _output_get "/Script/Engine.StaticMeshComponent")
      (bind _asprimitive_component_2 (Utilities|Casting|CastToPrimitiveComponent _array_element_2))
      (Collision|SetCollisionProfileName _asprimitive_component_2 "TFG_SpawnPhysics" true :!class /Script/Engine.PrimitiveComponent))
    (if (Class|VirtualHandComponentKismetLibrary|IsRight (Variables|Default|GetHand))
      (Variables|Default|SetHit (Collision|MakeHitResult false false 0.0 0.0 "0, 0, 0" (Transformation|GetWorldLocation (Variables|Default|GetRightHandSocket)) "0,0,1" "0,0,1" 0 0))
      (else
        (Variables|Default|SetHit (Collision|MakeHitResult false false 0.0 0.0 "0, 0, 0" (Transformation|GetWorldLocation (Variables|Default|GetLeftHandSocket)) "0,0,1" "0,0,1" 0 0))))
    (Class|TFGSGIPickup|Pickup(Message) (Variables|Default|GetSpawnedActor) false (Variables|Default|GetHit) false (Variables|Default|GetHand))))

(event EventOnActorReleased
  (params (Hand :type SG%20Virtual%20Hand%20Component%20Object%20Reference) (Actor :type Actor%20Object%20Reference))
  (Variables|Default|SetHand Hand)
  (Development|PrintString (Utilities|GetObjectName (Variables|Default|GetGrabbedActor)) true true "(R=0.779096,G=0.000000,B=1.000000,A=1.000000)" 2e+01)
  (Development|PrintString (Utilities|GetObjectName (Variables|Default|GetHand)) true true "(R=0.779096,G=0.000000,B=1.000000,A=1.000000)" 2e+01)
  (if (and (Utilities|IsValid (Variables|Default|GetSpawnedActor)) (Utilities|IsValid (Variables|Default|GetGrabbedActor)))
    (Class|TFGSGIPickup|Drop(Message) (Variables|Default|GetSpawnedActor) false)
    (Transformation|SetActorRotation (Variables|Default|GetGrabbedActor) (Transformation|GetWorldRotation (Variables|/Script/Engine.Actor|GetRootComponent (Variables|Default|GetSpawnedActor))) true)
    (Actor|DestroyActor (Variables|Default|GetSpawnedActor))
    (Rendering|SetActorHiddenInGame (Variables|Default|GetGrabbedActor) false)
    ;[1 1 1] Activar Colision Objeto invisible y de la mano
    (for _array_element (Actor|GetComponentsByClass (Variables|Default|GetGrabbedActor) "/Script/Engine.StaticMeshComponent")
      (bind _asprimitive_component (Utilities|Casting|CastToPrimitiveComponent _array_element))
      (Collision|SetCollisionProfileName _asprimitive_component "BlockAll" true :!class /Script/Engine.PrimitiveComponent))
    (Collision|SetCollisionProfileName (Variables|Default|GetHand) "BlockAll" true :!class /Script/Engine.PrimitiveComponent)
    (Collision|SetCollisionObjectType (Variables|Default|GetHand) "ECC_Pawn")
    (else
      (Development|PrintString "GrabbedActor or Spawned Actor noValid()" true true "(R=1.000000,G=0.000000,B=0.014578,A=1.000000)"))))

(fn ConstructionScript)