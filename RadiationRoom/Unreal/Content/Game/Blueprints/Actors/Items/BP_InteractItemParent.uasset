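; Parent Blueprint for interactable items with radiation contamination and database event logging.
; Interact and detection events fire event dispatchers, and a mesh hit against any actor with an AC_Radiation component marks the item contaminated.
; SendInteractEventToDB records timestamped user, scenario and item data through the DatabaseManager of either RR_GameInstance or RR_SG_GameInstance.
; BeginPlay binds database-close callbacks, whose handlers are empty stubs here.
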(event OnComponentHit(StaticMesh)
  (params (HitComponent :type Primitive%20Component%20Object%20Reference) (OtherActor :type Actor%20Object%20Reference) (OtherComp :type Primitive%20Component%20Object%20Reference) (NormalImpulse :type Vector :default "0, 0, 0") (Hit :type Hit%20Result%20Structure%20%28by%20ref%29))
  (Utilities|IsValid (Actor|GetComponentbyClass OtherActor "/Game/Game/Blueprints/Components/AC_Radiation.AC_Radiation_C")
    (:Is%20Valid
      (Variables|/Game/Game/Blueprints/Components/AC_Radiation.AC_Radiation_C|SetIsContamined? (Variables|Default|GetAC_Radiation) true))))

(event EventBeginPlay
  (bind _returnvalue (Game|GetGameInstance))
  (|CallParentFunction)
  (bind _asrr_game_instance (Utilities|Casting|CastToRR_GameInstance _returnvalue)
    (:then
      (Variables|Default|SetGameInstance _asrr_game_instance)
      (CallFunction|BindDatabaseEvents))
    (:CastFailed
      (bind _asrr_sg_game_instance (Utilities|Casting|CastToRR_SG_GameInstance _returnvalue))
      (Variables|Default|SetGameInstance _asrr_sg_game_instance)
      (CallFunction|BindDatabaseEvents))))

(event EventInteractwith
  (params (Player :type Pawn%20Object%20Reference))
  ;[1 1 1] Interact
  (Default|CallEDInteractionStarted))

(event EventCancelInteract
  (params (Player :type Pawn%20Object%20Reference))
  ;[1 1 1] Interact
  (Default|CallEDInteractionCompleted))

(event EventTick
  (params (DeltaSeconds :type Float%20%28single-precision%29)))

(event EventStartDetection
  (params (Player :type BP%20Player%20Object%20Reference))
  ;[1 1 1] Detection
  (Default|CallEDDetectionStarted))

(event EventStopDetection
  (params (Player :type BP%20Player%20Object%20Reference))
  ;[1 1 1] Detection
  (Default|CallEDDetectionCompleted))

(event Custom|SendInteractEventToDB
  (params (EventType :type E_ItemEventType%20Enum :default "NewEnumerator4"))
  (bind _returnvalue (Game|GetGameInstance))
  (bind _asrr_game_instance (Utilities|Casting|CastToRR_GameInstance _returnvalue)
    (:then
      (bind _data (Default|GetDataBaseMainInfoEvent _asrr_game_instance))
      (Default|SendItemInteractionEventtoDB (Variables|/Game/Game/Blueprints/RR_GameInstance.RR_GameInstance_C|GetDatabase%20Manager _asrr_game_instance) (Utilities|Struct|MakeF_ItemInteractionEvent 0 (.user_id (Utilities|Struct|BreakF_MainInfoEvent _data)) (Variables|/Game/Game/Blueprints/RR_GameInstance.RR_GameInstance_C|GetPlayerName _asrr_game_instance) (.scenario_type (Utilities|Struct|BreakF_MainInfoEvent _data)) (Variables|ItemInfo|GetActorId) (Variables|ItemInfo|GetItemType) EventType (Math|DateTime|Now))))
    (:CastFailed
      (bind _asrr_sg_game_instance (Utilities|Casting|CastToRR_SG_GameInstance _returnvalue))
      (bind _data_2 (Default|GetDataBaseMainInfoEvent _asrr_sg_game_instance))
      (Default|SendItemInteractionEventtoDB (Variables|/Game/TFG/TFG_SG_Template/Blueprints/RR_SG_GameInstance.RR_SG_GameInstance_C|GetDatabase%20Manager _asrr_sg_game_instance) (Utilities|Struct|MakeF_ItemInteractionEvent 0 (.user_id (Utilities|Struct|BreakF_MainInfoEvent _data_2)) (Variables|/Game/TFG/TFG_SG_Template/Blueprints/RR_SG_GameInstance.RR_SG_GameInstance_C|GetPlayerName _asrr_sg_game_instance) (.scenario_type (Utilities|Struct|BreakF_MainInfoEvent _data_2)) (Variables|ItemInfo|GetActorId) (Variables|ItemInfo|GetItemType) EventType (Math|DateTime|Now))))))

(event Custom|BindDatabaseEvents
  (EventDispatchers|AssignEDDatabaseNeedtobeClosed (Variables|Default|GetAC_Database) (delegate Custom|OnDatabaseNeedToBeClosed))
  (EventDispatchers|AssignEDDatabaseClosed (Variables|Default|GetAC_Database) (delegate Custom|OnDatabaseClosed)))

(event Custom|OnDatabaseNeedToBeClosed
  (CallFunction|SendLastEventstoDB))

(event Custom|OnDatabaseClosed)

(event Custom|SendLastEventsToDB)

(fn ConstructionScript)