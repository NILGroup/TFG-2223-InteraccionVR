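; Actor component that bridges its owner to the game instance's DatabaseManager for logging radiation-scenario events.
; On BeginPlay it caches either the RR or RR_SG game instance and re-broadcasts the manager's database closing and closed events through its own dispatchers.
; Send events package player dose arrays (only when an emission point exists), EPD dosimeter readings, or RBQ actor counts with user and scenario info for the manager.
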(event Custom|BindDatabaseEvents
  (bind _game_instance (Variables|Default|GetGame%20Instance))
  (bind _asrr_game_instance (Utilities|Casting|CastToRR_GameInstance _game_instance)
    (:then
      (bind _database_manager (Variables|/Game/Game/Blueprints/RR_GameInstance.RR_GameInstance_C|GetDatabase%20Manager _asrr_game_instance)
        (:then
          _)
        (:else)))
    (:CastFailed
      (bind _asrr_sg_game_instance (Utilities|Casting|CastToRR_SG_GameInstance _game_instance))
      (Variables|/Game/TFG/TFG_SG_Template/RR_SG_GameInstance.RR_SG_GameInstance_C|GetDatabase%20Manager _asrr_sg_game_instance
        (:then
          _)
        (:else))))
  (EventDispatchers|AssignEDDatabaseNeedtobeClosed _database_manager (delegate Custom|OnDatabaseNeedToBeClosed))
  (EventDispatchers|AssignEDDatabaseClosed _database_manager (delegate Custom|OnDatabaseClosed)))

(event Custom|OnDatabaseNeedToBeClosed
  (Default|CallEDDatabaseNeedtobeClosed))

(event Custom|OnDatabaseClosed
  (Default|CallEDDatabaseClosed))

(event EventBeginPlay
  (bind _returnvalue (Game|GetGameInstance))
  (Utilities|FlowControl|Sequence
    (:then_0
      (bind _asrr_game_instance (Utilities|Casting|CastToRR_GameInstance _returnvalue)
        (:then
          (Variables|Default|SetGame%20Instance _asrr_game_instance))
        (:CastFailed
          (bind _asrr_sg_game_instance (Utilities|Casting|CastToRR_SG_GameInstance _returnvalue))
          (Variables|Default|SetGame%20Instance _asrr_sg_game_instance)))
      (Variables|Default|SetOwner (Components|GetOwner)))
    (:then_1
      (CallFunction|BindDatabaseEvents))))

(event Custom|SendEPDRadiationEventToDB
  (bind _game_instance (Variables|Default|GetGame%20Instance))
  (bind _asrr_game_instance (Utilities|Casting|CastToRR_GameInstance _game_instance)
    (:then
      (bind _data (Default|GetDataBaseMainInfoEvent _asrr_game_instance))
      (bind _asbp_dosimeter_epd (Utilities|Casting|CastToBP_Dosimeter_EPD (Variables|Default|GetOwner)))
      (bind _database_manager (Variables|/Game/Game/Blueprints/RR_GameInstance.RR_GameInstance_C|GetDatabase%20Manager _asrr_game_instance)
        (:then
          (Default|SendEPDRadiationEventtoDB _database_manager (Utilities|Struct|MakeF_EPDRadiationEvent 0 (.user_id (Utilities|Struct|BreakF_MainInfoEvent _data)) (.scenario_type (Utilities|Struct|BreakF_MainInfoEvent _data)) (Variables|/Game/Game/Blueprints/Actors/Dosimeters/BP_Dosimeter_EPD.BP_Dosimeter_EPD_C|GetEPDId _asbp_dosimeter_epd) (Variables|/Game/Game/Blueprints/Actors/Dosimeters/BP_Dosimeter_EPD.BP_Dosimeter_EPD_C|GetCurrentEventDoseRateArray _asbp_dosimeter_epd) (Variables|/Game/Game/Blueprints/Actors/Dosimeters/BP_Dosimeter_EPD.BP_Dosimeter_EPD_C|GetCurrentEventDoseAbsortionArray _asbp_dosimeter_epd) (Variables|/Game/Game/Blueprints/Actors/Dosimeters/BP_Dosimeter_EPD.BP_Dosimeter_EPD_C|GetCurrentEventPositionArray _asbp_dosimeter_epd) (Variables|/Game/Game/Blueprints/Actors/Dosimeters/BP_Dosimeter_EPD.BP_Dosimeter_EPD_C|GetCurrentEventDatetimeArray _asbp_dosimeter_epd))))
        (:else)))
    (:CastFailed
      (bind _asrr_sg_game_instance (Utilities|Casting|CastToRR_SG_GameInstance _game_instance))
      (bind _data_2 (Default|GetDataBaseMainInfoEvent _asrr_sg_game_instance))
      (bind _asbp_dosimeter_epd_2 (Utilities|Casting|CastToBP_Dosimeter_EPD (Variables|Default|GetOwner)))
      (bind _database_manager_2 (Variables|/Game/TFG/TFG_SG_Template/RR_SG_GameInstance.RR_SG_GameInstance_C|GetDatabase%20Manager _asrr_sg_game_instance)
        (:then
          (Default|SendEPDRadiationEventtoDB _database_manager_2 (Utilities|Struct|MakeF_EPDRadiationEvent 0 (.user_id (Utilities|Struct|BreakF_MainInfoEvent _data_2)) (.scenario_type (Utilities|Struct|BreakF_MainInfoEvent _data_2)) (Variables|/Game/Game/Blueprints/Actors/Dosimeters/BP_Dosimeter_EPD.BP_Dosimeter_EPD_C|GetEPDId _asbp_dosimeter_epd_2) (Variables|/Game/Game/Blueprints/Actors/Dosimeters/BP_Dosimeter_EPD.BP_Dosimeter_EPD_C|GetCurrentEventDoseRateArray _asbp_dosimeter_epd_2) (Variables|/Game/Game/Blueprints/Actors/Dosimeters/BP_Dosimeter_EPD.BP_Dosimeter_EPD_C|GetCurrentEventDoseAbsortionArray _asbp_dosimeter_epd_2) (Variables|/Game/Game/Blueprints/Actors/Dosimeters/BP_Dosimeter_EPD.BP_Dosimeter_EPD_C|GetCurrentEventPositionArray _asbp_dosimeter_epd_2) (Variables|/Game/Game/Blueprints/Actors/Dosimeters/BP_Dosimeter_EPD.BP_Dosimeter_EPD_C|GetCurrentEventDatetimeArray _asbp_dosimeter_epd_2))))
        (:else)))))

(event Custom|SendRBQEventToDB
  (params (actor_id :type Array%20of%20Integers) (num_of_actors :type Array%20of%20Integers))
  (bind _game_instance (Variables|Default|GetGame%20Instance))
  (bind _asrr_game_instance (Utilities|Casting|CastToRR_GameInstance _game_instance)
    (:then
      (bind _data (Default|GetDataBaseMainInfoEvent _asrr_game_instance)))
    (:CastFailed
      (bind _asrr_sg_game_instance (Utilities|Casting|CastToRR_SG_GameInstance _game_instance))
      (Default|GetDataBaseMainInfoEvent _asrr_sg_game_instance)))
  (Default|SendRBQEventtoDB (Variables|/Game/Game/Blueprints/RR_GameInstance.RR_GameInstance_C|GetDatabase%20Manager _asrr_game_instance) (Utilities|Struct|MakeF_RBQEvent 0 (.user_id (Utilities|Struct|BreakF_MainInfoEvent _data)) (.scenario_type (Utilities|Struct|BreakF_MainInfoEvent _data)) actor_id num_of_actors (Math|DateTime|Now))))

(event Custom|SendUserRadiationEventToDB
  (bind _game_instance (Variables|Default|GetGame%20Instance))
  (bind _returnvalue (Actor|GetActorOfClass "/Game/Game/Blueprints/Actors/Radiation/BP_RadiationEmissionPoint.BP_RadiationEmissionPoint_C"))
  (Utilities|IsValid _returnvalue
    (:Is%20Valid
      (bind _asrr_game_instance (Utilities|Casting|CastToRR_GameInstance _game_instance)
        (:then
          (bind _data (Default|GetDataBaseMainInfoEvent _asrr_game_instance))
          (bind _asbp_player (Utilities|Casting|CastToBP_Player (Variables|Default|GetOwner)))
          (bind _database_manager (Variables|/Game/Game/Blueprints/RR_GameInstance.RR_GameInstance_C|GetDatabase%20Manager _asrr_game_instance)
            (:then
              (Default|SendUserRadiationEventtoDB _database_manager (Utilities|Struct|MakeF_UserRadiationEvent 0 (.user_id (Utilities|Struct|BreakF_MainInfoEvent _data)) (.scenario_type (Utilities|Struct|BreakF_MainInfoEvent _data)) (Variables|/Game/Game/Blueprints/Characters/Players/BP_Player.BP_Player_C|GetCurrentEventRadiationDoseRateArray _asbp_player) (Variables|/Game/Game/Blueprints/Characters/Players/BP_Player.BP_Player_C|GetCurrentEventDoseRadiationAbsortionArray _asbp_player) (Variables|/Game/Game/Blueprints/Characters/Players/BP_Player.BP_Player_C|GetCurrentEventRadiationPositionArray _asbp_player) (Variables|/Game/Game/Blueprints/Characters/Players/BP_Player.BP_Player_C|GetCurrentEventRadiationDatetimeArray _asbp_player))))
            (:else)))
        (:CastFailed
          (bind _asrr_sg_game_instance (Utilities|Casting|CastToRR_SG_GameInstance _game_instance))
          (bind _data_2 (Default|GetDataBaseMainInfoEvent _asrr_sg_game_instance))
          (bind _asbp_sg_player (Utilities|Casting|CastToBP_SG_Player (Variables|Default|GetOwner)))
          (bind _database_manager_2 (Variables|/Game/TFG/TFG_SG_Template/RR_SG_GameInstance.RR_SG_GameInstance_C|GetDatabase%20Manager _asrr_sg_game_instance)
            (:then
              (Default|SendUserRadiationEventtoDB _database_manager_2 (Utilities|Struct|MakeF_UserRadiationEvent 0 (.user_id (Utilities|Struct|BreakF_MainInfoEvent _data_2)) (.scenario_type (Utilities|Struct|BreakF_MainInfoEvent _data_2)) (Variables|/Game/TFG/TFG_SG_Template/Blueprints/BP_SG_Player.BP_SG_Player_C|GetCurrentEventRadiationDoseRateArray _asbp_sg_player) (Variables|/Game/TFG/TFG_SG_Template/Blueprints/BP_SG_Player.BP_SG_Player_C|GetCurrentEventDoseRadiationAbsortionArray _asbp_sg_player) (Variables|/Game/TFG/TFG_SG_Template/Blueprints/BP_SG_Player.BP_SG_Player_C|GetCurrentEventRadiationPositionArray _asbp_sg_player) (Variables|/Game/TFG/TFG_SG_Template/Blueprints/BP_SG_Player.BP_SG_Player_C|GetCurrentEventRadiationDatetimeArray _asbp_sg_player))))
            (:else)))))))