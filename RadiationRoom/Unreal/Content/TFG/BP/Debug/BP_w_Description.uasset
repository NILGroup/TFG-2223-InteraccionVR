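; Debug actor that shows a description through a w_Description widget hosted in its Widget component.
; On BeginPlay it casts the component's user widget and fills it from the actor's Text and Image variables.
; A valid Image becomes the widget's brush at the texture's size; otherwise the image element is collapsed.
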(event EventBeginPlay
  (bind _image (Variables|Default|GetImage))
  (bind _asw_description (Utilities|Casting|CastTow_Description (UserInterface|GetUserWidgetObject (Variables|Default|GetWidget))))
  (Utilities|IsValid _image
    (:Is%20Valid
      (Appearance|SetBrushfromTexture (Variables|/Game/TFG/Widgets/Debug/w_Description.w_Description_C|GetImage_130 _asw_description) _image true))
    (:Is%20Not%20Valid
      (Widget|SetVisibility (Variables|/Game/TFG/Widgets/Debug/w_Description.w_Description_C|GetImage_130 _asw_description) "Collapsed")))
  (Rendering|Components|TextRender|SetText (Variables|/Game/TFG/Widgets/Debug/w_Description.w_Description_C|GetText _asw_description) (Variables|Default|GetText)))

(event Collision|EventActorBeginOverlap
  (params (OtherActor :type Actor%20Object%20Reference)))

(event EventTick
  (params (DeltaSeconds :type Float%20%28single-precision%29)))

(fn ConstructionScript)