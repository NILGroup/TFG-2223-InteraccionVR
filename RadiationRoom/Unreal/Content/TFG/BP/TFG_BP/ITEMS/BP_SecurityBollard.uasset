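; Security bollard that a Rope can be strung between to form a chain of cordoned posts.
; Rope collision attaches it here and links the previous post's cable to this one, or, after a half-second lockout, detaches it and hands it back to that post.
; Each Tick stretches the Cable component toward the rope or next bollard, setting its length to the distance divided by 1.5.
; Attaching also calls a tape-attached event.
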(event Custom|RopeCollideWithPost
  (params (Rope :type BP%20Police%20Tape%20Object%20Reference))
  (if (and (!= (Variables|/Game/Game/Blueprints/Actors/Items/UsableItems/BP_PoliceTape.BP_PoliceTape_C|GetCurrentAttachedPost Rope) self) (not (Utilities|IsValid (Variables|Default|GetFromPost))))
    (Utilities|FlowControl|Sequence
      (:then_0
        (bind _currentattachedpost (Variables|/Game/Game/Blueprints/Actors/Items/UsableItems/BP_PoliceTape.BP_PoliceTape_C|GetCurrentAttachedPost Rope)
          (:then
            (if (!= _currentattachedpost self)
              (bind _output_get (Variables|Default|SetFromPost _currentattachedpost))
              (CallFunction|AttachRopeEnd _output_get self)))
          (:else)))
      (:then_1
        (CallFunction|AttachRopeStart Rope)
        (Default|SetCurrentPost Rope self)
        (Variables|Default|SetCanDetach false)
        (Utilities|FlowControl|Delay 0.5)
        (Variables|Default|SetCanDetach true))
      (:then_2
        (Default|CallEDTapeAttached self)))
    (elif (Variables|Default|GetCanDetach)
      (bind _currentattachedpost_2 (Variables|/Game/Game/Blueprints/Actors/Items/UsableItems/BP_PoliceTape.BP_PoliceTape_C|GetCurrentAttachedPost Rope)
        (:then
          (if (== _currentattachedpost_2 self)
            (Utilities|FlowControl|Sequence
              (:then_0
                (CallFunction|DetachRopeStart Rope))
              (:then_1
                (bind _frompost (Variables|Default|GetFromPost :!label _label)
                  (:then
                    (CallFunction|DetachRopeEnd _frompost Rope)
                    (Default|SetCurrentPost Rope (Variables|Default|GetFromPost))
                    (Variables|Default|SetFromPost 0))
                  (:else
                    (Default|SetCurrentPost Rope)))))))
        (:else
          (goto _label))))))

(event Custom|RopeEndMoving
  (bind _endactor (Variables|Default|GetEndActor))
  (bind _cable (Variables|Default|GetCable))
  (bind _cable_2 (Variables|Default|GetCable))
  (Utilities|IsValid _endactor
    (:Is%20Valid
      (Variables|/Script/CableComponent.CableComponent|SetbAttachEnd (Variables|Default|GetCable) true)
      (bind _asbp_security_bollard (Utilities|Casting|CastToBP_SecurityBollard _endactor)
        (:then
          (bind _endpoint (CallFunction|GetDistance (Variables|/Game/Game/Blueprints/Actors/Items/PlaceableItems/BP_SecurityBollard.BP_SecurityBollard_C|GetRopeInPole _asbp_security_bollard)))
          (bind _output_get (Variables|/Script/CableComponent.CableComponent|SetEndLocation _cable_2 (Math|Vector|MakeVector (.X (Math|Vector|BreakVector _endpoint)) (.Y (Math|Vector|BreakVector _endpoint)) 79.0)))
          (Variables|/Script/CableComponent.CableComponent|SetCableLength _cable_2 (/ (Math|Vector|VectorLength _output_get) 1.5)))
        (:CastFailed
          (bind _endpoint_2 (CallFunction|GetDistance (Variables|/Script/Engine.Actor|GetRootComponent _endactor)))
          (bind _output_get_2 (Variables|/Script/CableComponent.CableComponent|SetEndLocation _cable (+ _endpoint_2 "0.000000,0.000000,79.000000")))
          (Variables|/Script/CableComponent.CableComponent|SetCableLength _cable (/ (Math|Vector|VectorLength _output_get_2) 1.5)))))))

(event Custom|AttachRopeStart
  (params (Rope :type BP%20Police%20Tape%20Object%20Reference))
  (if (not (Variables|Default|GetRopeAttachedToStart))
    (Variables|Default|SetEndActor Rope)
    (Variables|Default|SetRopeAttachedToStart true)
    (Rendering|SetVisibility (Variables|Default|GetRopeInPole) true false)
    (Rendering|SetVisibility (Variables|Default|GetCable) true false)))

(event Custom|AttachRopeEnd
  (params (End%20Post :type BP%20Security%20Bollard%20Object%20Reference))
  (if (not (Variables|Default|GetRopeAttachedToEnd))
    (Variables|Default|SetRopeAttachedToEnd true)
    (Variables|Default|SetEndActor End%20Post)
    (Variables|Default|SetToPost End%20Post)))

(event Custom|DetachRopeStart
  (params (Rope :type BP%20Police%20Tape%20Object%20Reference))
  (Variables|Default|SetEndActor Rope)
  (Variables|Default|SetRopeAttachedToStart false)
  (Rendering|SetVisibility (Variables|Default|GetRopeInPole) false false)
  (Rendering|SetVisibility (Variables|Default|GetCable) false false))

(event Custom|DetachRopeEnd
  (params (Rope :type BP%20Police%20Tape%20Object%20Reference))
  (Variables|Default|SetEndActor Rope)
  (Variables|Default|SetToPost 0)
  (Variables|Default|SetRopeAttachedToEnd false))

(event EventBeginPlay
  (|CallParentFunction)
  (Rendering|SetVisibility (Variables|Default|GetRopeInPole) false false)
  (Rendering|SetVisibility (Variables|Default|GetCable) false false))

(event EventTick
  (params (DeltaSeconds :type Float%20%28single-precision%29))
  (|CallParentFunction DeltaSeconds)
  (CallFunction|RopeEndMoving))

(fn ConstructionScript)

(fn GetDistance
  (params (EndActor :type Scene%20Component%20Object%20Reference))
  (return (- (Transformation|GetWorldLocation EndActor) (Transformation|GetWorldLocation (Variables|Default|GetRopeInPole)))))