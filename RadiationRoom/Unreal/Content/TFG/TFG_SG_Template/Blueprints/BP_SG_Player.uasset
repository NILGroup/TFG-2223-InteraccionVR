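; Serious-game player Blueprint that handles inventory toggling, tutorial help and replicated item interaction, and logs player telemetry to a database.
; Self-rescheduling events sample movement distance and radiation dose while calculating exposure through ACRadiation.
; Completed moves are sent individually, while radiation samples are buffered in arrays, sent in batches and flushed when the database needs closing.
; Interact and cancel requests relay from server to multicast events that message the item.
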(event Custom|AddDistance
  (if (Variables|MovementEvent|GetIsMoving)
    (if (> (+ (Math|Vector|Distance(Vector) (Variables|MovementEvent|GetCurrent%20Position%20Move%20VW) (Transformation|GetWorldLocation (Variables|Default|GetMesh))) (Variables|MovementEvent|GetDistance%20Moved%20VW)) 5e+01)
      (Variables|MovementEvent|SetDistance%20Moved%20VW (+ (Math|Vector|Distance(Vector) (Variables|MovementEvent|GetCurrent%20Position%20Move%20VW) (Transformation|GetWorldLocation (Variables|Default|GetMesh))) (Variables|MovementEvent|GetDistance%20Moved%20VW)))
      (Variables|MovementEvent|SetCurrent%20Position%20Move%20VW (Transformation|GetWorldLocation (Variables|Default|GetMesh))))
    (Utilities|FlowControl|Delay 0.2)
    (CallFunction|AddDistance)))

(event Custom|MeasureRadiation
  (Default|CalculateRadiation (Variables|Default|GetAC_Radiation) (Utilities|Time|GetWorldDeltaSeconds))
  (CallFunction|SendUserRadiationEventtoDB)
  (Utilities|FlowControl|Delay 0.5)
  (CallFunction|MeasureRadiation))

(event Input|ActionEvents|InputActionDemandHelp
  (params (Key :type Key%20Structure :default "None"))
  (:Pressed
    (bind _tutorialmanager (Variables|Tutorial|GetTutorialManager)
      (:then
        (Default|DemandedCall _tutorialmanager))
      (:else))))

(event Input|ActionEvents|InputActionOpenCloseInventory
  (params (Key :type Key%20Structure :default "None"))
  (:Pressed
    (bind _asrr_game_instance (Utilities|Casting|CastToRR_GameInstance (Game|GetGameInstance)))
    (bind _state (Default|GetControlVar _asrr_game_instance "NewEnumerator12"))
    (if _state
      (if (Variables|Inventory|GetInventoryOpenned)
        (Variables|Inventory|SetInventoryOpenned false)
        (else
          (Variables|Inventory|SetInventoryOpenned true))))))

(event Custom|Interact%20With%20On%20Server
  (params (Look%20At%20Actor :type Actor%20Object%20Reference) (Player :type BP%20SG%20Player%20Object%20Reference))
  ;[1 1 1] Interact with
  (Utilities|IsValid Look%20At%20Actor
    (:Is%20Valid
      (CallFunction|InteractwithMulti Look%20At%20Actor Player))))

(event Custom|Interact%20With%20Multi
  (params (Look%20At%20Actor :type Actor%20Object%20Reference) (Player :type BP%20SG%20Player%20Object%20Reference))
  ;[1 1 1] Interact with
  (Utilities|IsValid Look%20At%20Actor
    (:Is%20Valid
      (Class|BIItemInteract|Interactwith(Message) Look%20At%20Actor Player))))

(event Custom|Cancel%20Multi
  (params (Item :type BP%20Interact%20Item%20Parent%20Object%20Reference) (Player :type BP%20SG%20Player%20Object%20Reference))
  ;[1 1 1] Cancel Interact
  (Class|BIItemInteract|CancelInteract(Message) Item Player))

(event Custom|Cancel%20On%20Server
  (params (Item :type BP%20Interact%20Item%20Parent%20Object%20Reference) (Player :type BP%20SG%20Player%20Object%20Reference))
  ;[1 1 1] Cancel Interact
  (CallFunction|CancelMulti Item Player))

(event Custom|SendUserInputEventToDB
  (params (input_type :type String) (input_state :type E_UserInputState%20Enum :default "NewEnumerator0"))
  (bind _data (Default|GetDataBaseMainInfoEvent (Variables|Default|GetGameInstance)))
  (bind _database_manager (Variables|/Game/TFG/TFG_SG_Template/Blueprints/RR_SG_GameInstance.RR_SG_GameInstance_C|GetDatabase%20Manager (Variables|Default|GetGameInstance))
    (:then
      (Default|SendSGUserInputEventtoDB _database_manager (Utilities|Struct|MakeF_SG_UserInputEvent 0 (.user_id (Utilities|Struct|BreakF_MainInfoEvent _data)) (.scenario_type (Utilities|Struct|BreakF_MainInfoEvent _data)) input_type input_state (Math|DateTime|Now))))
    (:else)))

(event Custom|SendUserRadiationEventToDB
  (bind _ac_radiation (Variables|Default|GetAC_Radiation))
  (bind _returnvalue (Actor|GetActorOfClass "/Game/Game/Blueprints/Actors/Radiation/BP_RadiationEmissionPoint.BP_RadiationEmissionPoint_C"))
  (Utilities|IsValid _returnvalue
    (:Is%20Valid
      (Utilities|Array|Add (Variables|DatabaseData|GetCurrentEventRadiationDoseRateArray) (Variables|/Game/Game/Blueprints/Components/AC_Radiation.AC_Radiation_C|GetDoseRate _ac_radiation))
      (Utilities|Array|Add (Variables|DatabaseData|GetCurrentEventDoseRadiationAbsortionArray) (Variables|/Game/Game/Blueprints/Components/AC_Radiation.AC_Radiation_C|GetDoseAbsorption _ac_radiation))
      (Utilities|Array|Add (Variables|DatabaseData|GetCurrentEventRadiationPositionArray) (Transformation|GetActorLocation))
      (bind _returnvalue_2 (Utilities|Array|Add (Variables|DatabaseData|GetCurrentEventRadiationDatetimeArray) (Math|DateTime|Now)))
      (if (>= _returnvalue_2 9)
        (CallFunction|SendEventstoDB)))))

(event Custom|OnDatabaseNeedToBeClosed
  (CallFunction|SendLastEventstoDB))

(event Custom|OnDatabaseClosed)

(event Custom|SendLastEventsToDB
  (Default|SendUserRadiationEventtoDB (Variables|Default|GetAC_Database))
  (Utilities|Array|Clear (Variables|DatabaseData|GetCurrentEventRadiationDoseRateArray))
  (Utilities|Array|Clear (Variables|DatabaseData|GetCurrentEventDoseRadiationAbsortionArray))
  (Utilities|Array|Clear (Variables|DatabaseData|GetCurrentEventRadiationPositionArray))
  (Utilities|Array|Clear (Variables|DatabaseData|GetCurrentEventRadiationDatetimeArray)))

(event Custom|BindDataBaseEvents
  (EventDispatchers|AssignEDDatabaseNeedtobeClosed (Variables|Default|GetAC_Database) (delegate Custom|OnDatabaseNeedToBeClosed))
  (EventDispatchers|AssignEDDatabaseClosed (Variables|Default|GetAC_Database) (delegate Custom|OnDatabaseClosed)))

(event Custom|SendEventsToDB
  (Default|SendUserRadiationEventtoDB (Variables|Default|GetAC_Database))
  (Utilities|Array|Clear (Variables|DatabaseData|GetCurrentEventRadiationDoseRateArray))
  (Utilities|Array|Clear (Variables|DatabaseData|GetCurrentEventDoseRadiationAbsortionArray))
  (Utilities|Array|Clear (Variables|DatabaseData|GetCurrentEventRadiationPositionArray))
  (Utilities|Array|Clear (Variables|DatabaseData|GetCurrentEventRadiationDatetimeArray)))

(event Custom|SendMoveEventToDB
  (params (move_type :type E_MovementType%20Enum :default "NewEnumerator0") (start_datetime :type Date%20Time%20Structure) (end_datetime :type Date%20Time%20Structure) (start_position :type Vector) (end_position :type Vector) (distance :type Float%20%28double-precision%29))
  (bind _data (Default|GetDataBaseMainInfoEvent (Variables|Default|GetGameInstance)))
  (bind _database_manager (Variables|/Game/TFG/TFG_SG_Template/Blueprints/RR_SG_GameInstance.RR_SG_GameInstance_C|GetDatabase%20Manager (Variables|Default|GetGameInstance))
    (:then
      (Default|SendMoveEventtoDB _database_manager (Utilities|Struct|MakeF_MoveEvent 0 (.user_id (Utilities|Struct|BreakF_MainInfoEvent _data)) (.scenario_type (Utilities|Struct|BreakF_MainInfoEvent _data)) move_type start_datetime end_datetime start_position end_position distance)))
    (:else)))

(event Custom|UserStopMovingInVirtualWorld
  (if (Variables|MovementEvent|GetIsMoving)
    (Utilities|FlowControl|Sequence
      (:then_0
        (Variables|MovementEvent|SetIsMoving false)
        (Variables|MovementEvent|SetEnd%20Datetime%20Move%20VW (Math|DateTime|Now))
        (Variables|MovementEvent|SetEnd%20Position%20Move%20VW (Transformation|GetWorldLocation (Variables|Default|GetMesh)))
        (Variables|MovementEvent|SetDistance%20Moved%20VW (+ (Math|Vector|Distance(Vector) (Variables|MovementEvent|GetCurrent%20Position%20Move%20VW) (Variables|MovementEvent|GetEnd%20Position%20Move%20VW)) (Variables|MovementEvent|GetDistance%20Moved%20VW))))
      (:then_1
        (CallFunction|SendMoveEventtoDB "NewEnumerator1" (Variables|MovementEvent|GetStart%20Datetime%20Move%20VW) (Variables|MovementEvent|GetEnd%20Datetime%20Move%20VW) (Variables|MovementEvent|GetStart%20Position%20Move%20VW) (Variables|MovementEvent|GetEnd%20Position%20Move%20VW) (/ (Variables|MovementEvent|GetDistance%20Moved%20VW) 1e+02))))))

(event Custom|UserStartMovingInVirtualWorld
  (if (not (Variables|MovementEvent|GetIsMoving))
    (Variables|MovementEvent|SetIsMoving true)
    (Variables|MovementEvent|SetStart%20Datetime%20Move%20VW (Math|DateTime|Now))
    (bind _output_get (Variables|MovementEvent|SetStart%20Position%20Move%20VW (Transformation|GetWorldLocation (Variables|Default|GetMesh))))
    (Variables|MovementEvent|SetCurrent%20Position%20Move%20VW _output_get)
    (Variables|MovementEvent|SetDistance%20Moved%20VW 0.0)
    (CallFunction|AddDistance)))

(fn ConstructionScript)