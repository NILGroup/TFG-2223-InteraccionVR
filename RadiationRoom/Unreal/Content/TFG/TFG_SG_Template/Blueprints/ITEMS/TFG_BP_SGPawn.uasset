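; SenseGlove VR pawn that handles two-handed object grabbing and gesture-based teleporting.
; On grab, it hides the original and spawns a class-mapped pickup proxy attached to the hand, using collision profiles to separate them.
; Release copies the proxy's rotation to the original, restores it and destroys the proxy.
; Each tick, a left-hand pistol pose traces along device rotation to highlight teleport targets; dropping the pose teleports there.
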(event EventOnGrabStateUpdated
  (params (GrabState :type SG%20Grab%20State%20Structure%20%28by%20ref%29))
  ;[1 1 1] DoubleHanded
  (if (not (Class|SGDeviceKismetLibrary|IsConnected (Class|VirtualHandComponentKismetLibrary|GetConnectedGlove (.Hand (Utilities|Struct|BreakSGGrabState GrabState)))))
    (bind _output_get (Variables|Default|SetHand (stale EventOnActorReleased Hand)))
    (if (Class|VirtualHandComponentKismetLibrary|IsRight _output_get)
      ;;[1 1 1] OnActorReleased
      (Variables|Default|SetGrabbedActor (Variables|Default|GetGrabbedActor_Right))
      (Variables|Default|SetSpawnedActor (Variables|Default|GetSpawnedActor_Right))
      (else
        (Variables|Default|SetGrabbedActor (Variables|Default|GetGrabbedActor_Left))
        (Variables|Default|SetSpawnedActor (Variables|Default|GetSpawnedActor_Left))))
    ;;;[1 1 1] Comprobar si es valida la llamada OnActorReleased
    (if (Utilities|IsValid (Variables|Default|GetSpawnedActor))
      (if (Utilities|IsValid (Variables|Default|GetGrabbedActor))
        (if (Utilities|IsValid (Variables|Default|GetHand))
          ;;;[1 1 1] Settear la rotacion de GrabbedActor con la de SpawnedActor y quitar la invisibilidad de GrabbedActor
          (Transformation|SetActorRotation (Variables|Default|GetGrabbedActor) (Transformation|GetWorldRotation (Variables|/Script/Engine.Actor|GetRootComponent (Variables|Default|GetSpawnedActor))) true)
          (Rendering|SetActorHiddenInGame (Variables|Default|GetGrabbedActor) false)
          ;;;[1 1 1] Activar Colision Objeto invisible y de la mano
          (for _array_element (Actor|GetComponentsByClass (Variables|Default|GetGrabbedActor) "/Script/Engine.StaticMeshComponent")
            (bind _asprimitive_component (Utilities|Casting|CastToPrimitiveComponent _array_element))
            (Collision|SetCollisionProfileName _asprimitive_component "BlockAll" true :!class /Script/Engine.PrimitiveComponent))
          (Collision|SetCollisionProfileName (Variables|Default|GetHand) "BlockAll" true :!class /Script/Engine.PrimitiveComponent)
          (Collision|SetCollisionObjectType (Variables|Default|GetHand) "ECC_Pawn")
          (Class|TFGSGIPickup|Drop(Message) (Variables|Default|GetSpawnedActor) false)
          ;;;[1 1 1] Eliminar las referencias de los objetos SpawnedActor y Grabbed Actor
          (Actor|DestroyActor (Variables|Default|GetSpawnedActor))
          (Variables|Default|SetSpawnedActor 0)
          (Variables|Default|SetGrabbedActor 0)
          (Variables|Default|SetLastGrabbedActor 0)
          (if (Class|VirtualHandComponentKismetLibrary|IsRight (Variables|Default|GetHand))
            (Variables|Default|SetGrabbedActor_Right 0)
            (Variables|Default|SetSpawnedActor_Right 0)
            (else
              (Variables|Default|SetGrabbedActor_Left 0)
              (Variables|Default|SetSpawnedActor_Left 0)))
          (Development|PrintString "Drop()" true true "(R=0.038153,G=1.000000,B=0.000000,A=1.000000)"))))))

(event Collision|EventActorBeginOverlap
  (params (OtherActor :type Actor%20Object%20Reference)))

(event EventOnActorGrabbed
  (params (Hand :type SG%20Virtual%20Hand%20Component%20Object%20Reference) (Actor :type Actor%20Object%20Reference))
  ;[1 1 1] DoubleHanded
  ;;[1 1 1] OnActorGrabbed
  ;;;[1 1 1] Diferenciar entre mano izquierda y derecha
  (bind _output_get (Variables|Default|SetHand Hand))
  (Variables|Default|SetGrabbedActor Actor)
  (if (Class|VirtualHandComponentKismetLibrary|IsRight _output_get)
    (Variables|Default|SetGrabbedActor_Right (Variables|Default|GetGrabbedActor))
    (else
      (Variables|Default|SetGrabbedActor_Left (Variables|Default|GetGrabbedActor))))
  ;;;[1 1 1] Comprobar si es valida la llamada OnActorGrabbed
  (if (not (== (Variables|Default|GetGrabbedActor) (Variables|Default|GetLastGrabbedActor)))
    (if (Utilities|IsValid (Variables|Default|GetGrabbedActor))
      (if (Utilities|IsValid (Variables|Default|GetHand))
        ;;;[1 1 1] Settear el Hit (posicion donde se atachea el objeto que vamos a spawnear)
        (if (Class|VirtualHandComponentKismetLibrary|IsRight (Variables|Default|GetHand))
          (Variables|Default|SetHit (Collision|MakeHitResult false false 0.0 0.0 "0, 0, 0" (Transformation|GetWorldLocation (Variables|Default|GetRightHandSocket)) "0,0,1" "0,0,1" 0 0))
          (else
            (Variables|Default|SetHit (Collision|MakeHitResult false false 0.0 0.0 "0, 0, 0" (Transformation|GetWorldLocation (Variables|Default|GetLeftHandSocket)) "0,0,1" "0,0,1" 0 0))))
        ;;;[1 1 1] Cambiar perfil de colisiones de Grabbed Actor (para que solo colisione con la mano) y hacerlo invisible
        (Variables|Default|SetLastGrabbedActor (Variables|Default|GetGrabbedActor))
        (for _array_element (Actor|GetComponentsByClass (Variables|Default|GetGrabbedActor) "/Script/Engine.StaticMeshComponent")
          (bind _asprimitive_component (Utilities|Casting|CastToPrimitiveComponent _array_element))
          (Collision|SetCollisionProfileName _asprimitive_component "TFG_GrabCollissions" true :!class /Script/Engine.PrimitiveComponent)
          ;;;[1 1 1] Settear SpawnedActor y cambiarle el perfil de colisiones para que no colisione con el GrabbedObject ni con la mano
          (bind _output_class (Utilities|GrabbedClassType (Utilities|GetClass (Variables|Default|GetGrabbedActor)))
            (:End
              (bind _returnvalue (Game|SpawnActorfromClass _output_class (Transformation|GetActorTransform (Variables|Default|GetGrabbedActor)) "Undefined" "OverrideRootScale" 0 0))
              (Variables|Default|SetSpawnedActor _returnvalue)
              (if (Class|VirtualHandComponentKismetLibrary|IsRight (Variables|Default|GetHand))
                (Variables|Default|SetSpawnedActor_Right (Variables|Default|GetSpawnedActor))
                (else
                  (Variables|Default|SetSpawnedActor_Left (Variables|Default|GetSpawnedActor))))
              (for _array_element_2 (Actor|GetComponentsByClass (Variables|Default|GetSpawnedActor) "/Script/Engine.StaticMeshComponent")
                (bind _asprimitive_component_2 (Utilities|Casting|CastToPrimitiveComponent _array_element_2))
                (Collision|SetCollisionProfileName _asprimitive_component_2 "TFG_SpawnPhysics" true :!class /Script/Engine.PrimitiveComponent)
                (Class|TFGSGIPickup|Pickup(Message) (Variables|Default|GetSpawnedActor) false (Variables|Default|GetHit) false (Variables|Default|GetHand) false)
                (Development|PrintString "Pickup()")))))
        (Rendering|SetActorHiddenInGame (Variables|Default|GetGrabbedActor) true)))))

(event EventOnActorReleased
  (params (Hand :type SG%20Virtual%20Hand%20Component%20Object%20Reference) (Actor :type Actor%20Object%20Reference))
  ;[1 1 1] DoubleHanded
  (bind _output_get (Variables|Default|SetHand Hand))
  (if (Class|VirtualHandComponentKismetLibrary|IsRight _output_get)
    ;;[1 1 1] OnActorReleased
    (Variables|Default|SetGrabbedActor (Variables|Default|GetGrabbedActor_Right))
    (Variables|Default|SetSpawnedActor (Variables|Default|GetSpawnedActor_Right))
    (else
      (Variables|Default|SetGrabbedActor (Variables|Default|GetGrabbedActor_Left))
      (Variables|Default|SetSpawnedActor (Variables|Default|GetSpawnedActor_Left))))
  ;;;[1 1 1] Comprobar si es valida la llamada OnActorReleased
  (if (Utilities|IsValid (Variables|Default|GetSpawnedActor))
    (if (Utilities|IsValid (Variables|Default|GetGrabbedActor))
      (if (Utilities|IsValid (Variables|Default|GetHand))
        ;;;[1 1 1] Settear la rotacion de GrabbedActor con la de SpawnedActor y quitar la invisibilidad de GrabbedActor
        (Transformation|SetActorRotation (Variables|Default|GetGrabbedActor) (Transformation|GetWorldRotation (Variables|/Script/Engine.Actor|GetRootComponent (Variables|Default|GetSpawnedActor))) true)
        (Rendering|SetActorHiddenInGame (Variables|Default|GetGrabbedActor) false)
        ;;;[1 1 1] Activar Colision Objeto invisible y de la mano
        (for _array_element (Actor|GetComponentsByClass (Variables|Default|GetGrabbedActor) "/Script/Engine.StaticMeshComponent")
          (bind _asprimitive_component (Utilities|Casting|CastToPrimitiveComponent _array_element))
          (Collision|SetCollisionProfileName _asprimitive_component "BlockAll" true :!class /Script/Engine.PrimitiveComponent))
        (Collision|SetCollisionProfileName (Variables|Default|GetHand) "BlockAll" true :!class /Script/Engine.PrimitiveComponent)
        (Collision|SetCollisionObjectType (Variables|Default|GetHand) "ECC_Pawn")
        (Class|TFGSGIPickup|Drop(Message) (Variables|Default|GetSpawnedActor) false)
        ;;;[1 1 1] Eliminar las referencias de los objetos SpawnedActor y Grabbed Actor
        (Actor|DestroyActor (Variables|Default|GetSpawnedActor))
        (Variables|Default|SetSpawnedActor 0)
        (Variables|Default|SetGrabbedActor 0)
        (Variables|Default|SetLastGrabbedActor 0)
        (if (Class|VirtualHandComponentKismetLibrary|IsRight (Variables|Default|GetHand))
          (Variables|Default|SetGrabbedActor_Right 0)
          (Variables|Default|SetSpawnedActor_Right 0)
          (else
            (Variables|Default|SetGrabbedActor_Left 0)
            (Variables|Default|SetSpawnedActor_Left 0)))
        (Development|PrintString "Drop()" true true "(R=0.038153,G=1.000000,B=0.000000,A=1.000000)")))))

(event EventTick
  (params (DeltaSeconds :type Float%20%28single-precision%29))
  (bind _returnvalue (Transformation|GetActorLocation))
  (bind _returnvalue_2 (+ _returnvalue "0.000000,0.000000,100.000000"))
  ;[1 1 1] Detección de pose de la mano
  (bind _pose (CallFunction|DetectPose false))
  (switch Utilities|FlowControl|Switch|SwitchonHandPoses _pose
    (:NewEnumerator1
      ;[1 1 1] Pose pistola: Buscar la posicion de teletrasporte
      (bind (_outhit _returnvalue_3) (Collision|LineTraceForObjects _returnvalue_2 (+ _returnvalue_2 (* (Math|Vector|GetForwardVector (.DeviceRotation (Class|HeadMountedDisplayFunctionLibrary|GetOrientationandPosition))) (Variables|Default|GetRaycastDistance))) (Variables|Default|GetTeleportDest) false 0 "ForDuration" true "(R=1.000000,G=0.000000,B=0.000000,A=1.000000)" "(R=0.000000,G=1.000000,B=0.000000,A=1.000000)" 1.0))
      (if _returnvalue_3
        ;;[1 1 1] Guardado de la posicion destino
        (if (not (== (.HitActor (Collision|BreakHitResult _outhit)) 0))
          (Variables|Default|SetTeleport_pos (Transformation|GetActorLocation (.HitActor (Collision|BreakHitResult _outhit))))
          ;;[1 1 1] Cambio de color del punto que se  ha detectado y quita el color de los anteriores
          (bind _asstatic_mesh_actor (Utilities|Casting|CastToStaticMeshActor (.HitActor (Collision|BreakHitResult _outhit)))
            (:then
              (bind _mesh_reference_teleport (Variables|Default|GetMesh%20reference%20teleport)
                (:then
                  (Rendering|Material|SetMaterial (Variables|/Script/Engine.StaticMeshActor|GetStaticMeshComponent _mesh_reference_teleport) 0 "/Game/TFG/TFG_SG_Template/Materials/M_Teleport.M_Teleport"))
                (:else
                  _))
              (bind _output_get (Variables|Default|SetMesh%20reference%20teleport _asstatic_mesh_actor))
              (Rendering|Material|SetMaterial (Variables|/Script/Engine.StaticMeshActor|GetStaticMeshComponent _output_get) 0 "/Game/TFG/TFG_SG_Template/Materials/M_Teleport_rojo.M_Teleport_rojo"))
            (:CastFailed
              (bind _mesh_reference_teleport_2 (Variables|Default|GetMesh%20reference%20teleport)
                (:then
                  (Rendering|Material|SetMaterial (Variables|/Script/Engine.StaticMeshActor|GetStaticMeshComponent _mesh_reference_teleport_2) 0 "/Game/TFG/TFG_SG_Template/Materials/M_Teleport.M_Teleport"))
                (:else)))))))
    (:NewEnumerator2
      ;[1 1 1] Sin posicion: intenta teletrasportar
      ;;[1 1 1] Teletransportacion
      (if (not (Utilities|Operators|EqualEqual (Variables|Default|GetTeleport_pos) "-100.000000,-100.000000,-100.000000" 0.0))
        (Transformation|Teleport (Variables|Default|GetTeleport_pos) "0, 0, 0")
        (Variables|Default|SetTeleport_pos "-100.000000,-100.000000,-100.000000")))))

(fn ConstructionScript)

(fn DetectPose
  (params (Right :type Boolean))
  (bind _self self)
  (bind _self_2 self)
  (bind _returnvalue (Class|PawnKismetLibrary|GetRealHandRight _self))
  (bind _returnvalue_2 (Class|PawnKismetLibrary|GetRealHandLeft _self_2))
  (if Right
    (if (Class|VirtualHandComponentKismetLibrary|IsGloveConnected _returnvalue)
      (bind _returnvalue_3 (Class|VirtualHandComponentKismetLibrary|GetHandPose _returnvalue))
      (bind _pose (CallFunction|GetOneHandPose (Class|SGHandPoseKismetLibrary|GetNormalizedFlexionFBC01 _returnvalue_3 "Thumb" true) (Class|SGHandPoseKismetLibrary|GetNormalizedFlexionFBC01 _returnvalue_3 "Index" true) (Class|SGHandPoseKismetLibrary|GetNormalizedFlexionFBC01 _returnvalue_3 "Middle" true) (Class|SGHandPoseKismetLibrary|GetNormalizedFlexionFBC01 _returnvalue_3 "Ring" true)))
      (return _pose)
      (else
        _))
    (elif (Class|VirtualHandComponentKismetLibrary|IsGloveConnected _returnvalue_2)
      (bind _returnvalue_4 (Class|VirtualHandComponentKismetLibrary|GetHandPose _returnvalue_2))
      (bind _pose_2 (CallFunction|GetOneHandPose (Class|SGHandPoseKismetLibrary|GetNormalizedFlexionFBC01 _returnvalue_4 "Thumb" true) (Class|SGHandPoseKismetLibrary|GetNormalizedFlexionFBC01 _returnvalue_4 "Index" true) (Class|SGHandPoseKismetLibrary|GetNormalizedFlexionFBC01 _returnvalue_4 "Middle" true) (Class|SGHandPoseKismetLibrary|GetNormalizedFlexionFBC01 _returnvalue_4 "Ring" true)))
      (return _pose_2)
      (else
        _)))
  (return "NewEnumerator2"))

(fn GetOneHandPose
  (params (ThumbFlex :type Float%20%28double-precision%29) (IndexFlex :type Float%20%28double-precision%29) (MiddleFlex :type Float%20%28double-precision%29) (RingFlex :type Float%20%28double-precision%29))
  ;[1 1 1] Fist
  (Math|Float|CompareFloat ThumbFlex 0.5
    (:>
      _)
    (:==
      _)
    (:<
      _))
  (Math|Float|CompareFloat ThumbFlex 0.4
    (:>
      _)
    (:==
      (Math|Float|CompareFloat IndexFlex 0.4 :!label _label
        (:>
          _)
        (:==
          (Math|Float|CompareFloat MiddleFlex 0.5 :!label _label_2
            (:>
              (return "NewEnumerator1"))
            (:==
              _)
            (:<
              _)))
        (:<
          (goto _label_2))))
    (:<
      (goto _label)))
  (return "NewEnumerator2"))