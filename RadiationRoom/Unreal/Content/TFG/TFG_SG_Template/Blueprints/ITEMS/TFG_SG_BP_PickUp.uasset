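; Base physics pickup actor that can be grabbed, carried on an attach component's HandSocket, and dropped or thrown.
; Pickup binds MainMesh to Root through a physics constraint, with Accurate and loose modes and optional inertia damping; drop restores saved collision responses.
; Hits while held briefly free the constraint's linear limits.
; An optional SweepMesh copy stands in for wall pass-through, though its sweep-follow update is unconnected and Tick is empty.
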(event Custom|HitCustom
  (params (HitComponent :type Primitive%20Component%20Object%20Reference) (OtherActor :type Actor%20Object%20Reference) (OtherComp :type Primitive%20Component%20Object%20Reference) (NormalImpulse :type Vector) (Hit :type Hit%20Result%20Structure%20%28by%20ref%29))
  (bind _physicsconstraint (Variables|Default|GetPhysicsConstraint))
  ;[1 1 1] Hit
  (if (not (Variables|Default|GetIgnoreHit?))
    (if (Variables|Default|GetAttach)
      (Variables|Default|SetHitActive true)
      (Class|PhysicsConstraintComponent|SetLinearXLimit _physicsconstraint "LCM_Free" 0.0)
      (Class|PhysicsConstraintComponent|SetLinearYLimit _physicsconstraint "LCM_Free" 0.0)
      (Class|PhysicsConstraintComponent|SetLinearZLimit _physicsconstraint "LCM_Free" 0.0)
      (CallFunction|Free)
      (Utilities|FlowControl|RetriggerableDelay (Variables|Tunemeup|GetRecoveryFromHit))
      (Utilities|FlowControl|Sequence
        (:then_0
          (Class|PhysicsConstraintComponent|SetLinearXLimit _physicsconstraint "LCM_Locked" 0.0)
          (Class|PhysicsConstraintComponent|SetLinearYLimit _physicsconstraint "LCM_Locked" 0.0)
          (Class|PhysicsConstraintComponent|SetLinearZLimit _physicsconstraint "LCM_Locked" 0.0)
          (CallFunction|Lock)
          (Variables|Default|SetHitActive false))))))

(event Custom|CustomAttach
  (bind _attachtransform (Variables|Default|GetAttachTransform))
  (bind _attachtransform_2 (Variables|Default|GetAttachTransform))
  (bind _attachtransform_3 (Variables|Default|GetAttachTransform))
  (bind _mainmesh (Variables|Default|GetMainMesh))
  (bind _mainmesh_2 (Variables|Default|GetMainMesh))
  (bind _inttransform (Variables|Default|GetIntTransform))
  (bind _mainmesh_3 (Variables|Default|GetMainMesh))
  (bind _mainmesh_4 (Variables|Default|GetMainMesh))
  (bind _returnvalue (Transformation|GetWorldLocation _attachtransform_2))
  ;[1 1 1] Pickup
  (Variables|Default|SetAttach true)
  (Input|EnableInput (Game|GetPlayerController 0))
  (Utilities|IsValid (Variables|Default|GetPhysicsConstraint)
    (:Is%20Valid
      ;;[1 1 1] For stability.
      (if (or (Physics|IsSimulatingPhysics _mainmesh "None") (Variables|Default|GetRotate))
        _
        (else
          (Utilities|FlowControl|Delay 0.0)
          (Physics|SetSimulatePhysics _mainmesh true)))
      (Utilities|FlowControl|Sequence
        (:then_0
          (Class|PhysicsConstraintComponent|BreakConstraint (Variables|Default|GetPhysicsConstraint))
          ;;[1 1 1] Memorise the default collision
          (Utilities|Array|Clear (Variables|Default|GetIntCollision))
          (bind _enumvalue (|ForEachECollisionChannel)
            (:LoopBody
              (Utilities|Array|Add (Variables|Default|GetIntCollision) (Collision|GetCollisionResponsetoChannel (Variables|Default|GetMainMesh) _enumvalue)))
            (:then
              (Collision|SetCollisionResponsetoChannel (Variables|Default|GetMainMesh) "ECC_Pawn" "ECR_Ignore")
              (Variables|Default|SetBeforeAction (Transformation|GetWorldTransform (Variables|Default|GetMainMesh)))
              (Variables|/Script/Engine.SceneComponent|SetbAbsoluteLocation (Variables|Default|GetMainMesh) true)
              (Variables|/Script/Engine.SceneComponent|SetbAbsoluteLocation (Variables|Default|GetPhysicsConstraint) true)
              (if (Variables|Tunemeup|GetFixWallPassThrough)
                (Variables|Default|SetTickForSweep true)
                (Rendering|SetVisibility (Variables|Default|GetSweepMesh) false false))
              (if (Variables|TuneMeUp|GetAccurate)
                ;;[0 0 0] Accurate
                (if (Variables|Default|GetRotate)
                  (Transformation|SetWorldLocationAndRotation _mainmesh_3 (.location (Variables|Default|GetLast)) (.rotation (Variables|Default|GetLast)) false true)
                  (Collision|SetCollisionResponsetoAllChannels _mainmesh_3 "ECR_Overlap") ; To prevent nearby meshes from flying off
                )
                (Transformation|SetWorldLocation (Variables|Default|GetRoot) (.ImpactPoint (Collision|BreakHitResult (Variables|Default|GetHitClick))) false true)
                (Physics|SetSimulatePhysics _mainmesh_2 true)
                (Class|PhysicsConstraintComponent|SetConstrainedComponents (Variables|Default|GetPhysicsConstraint) (Variables|Default|GetRoot) "None" _mainmesh_2 "None")
                (if (Variables|Default|GetRotate)
                  ;;;[1 1 1] Solves a lot of problems when returning from inspection
                  (Transformation|SetWorldLocation (Variables|Default|GetPhysicsConstraint) (+ _returnvalue (* (Math|Vector|GetForwardVector _attachtransform_2) (Math|Vector|Distance(Vector) _returnvalue (.location (Variables|Default|GetBeforeAction))))) false true)
                  (else
                    (Transformation|AttachComponentToComponent (Variables|Default|GetRoot) _attachtransform "HandSocket" "KeepWorld" "KeepWorld" "KeepWorld" true)
                    (Transformation|AttachComponentToComponent (Variables|Default|GetPhysicsConstraint) _attachtransform "HandSocket" "KeepWorld" "KeepWorld" "KeepWorld" true)))
                (Utilities|FlowControl|Sequence
                  (:then_0
                    (if (Variables|Default|GetRotate)
                      ;;;[1 1 1] Returning from where you got it
                      (Utilities|FlowControl|Delay 0.0)
                      (Transformation|SetWorldLocationAndRotation (Variables|Default|GetMainMesh) (.location (Variables|Default|GetBeforeAction)) (.rotation (Variables|Default|GetBeforeAction)) false true)
                      (Utilities|DefaultCollision)
                      (Collision|SetCollisionResponsetoChannel (Variables|Default|GetMainMesh) "ECC_Pawn" "ECR_Ignore")
                      (else
                        (Variables|Default|SetLast (Transformation|GetWorldTransform (Variables|Default|GetMainMesh)))))))
                (else
                  ;;[1 1 1] Ignore other physical subjects.
                  (if (Variables|Tunemeup|GetIgnoreCamera?)
                    _
                    (else
                      (Collision|SetCollisionResponsetoChannel (Variables|Default|GetMainMesh) "ECC_PhysicsBody" "ECR_Ignore")))
                  (Transformation|SetWorldLocation (Variables|Default|GetRoot) (.ImpactPoint (Collision|BreakHitResult (Variables|Default|GetHitClick))) false true)
                  (Transformation|AttachComponentToComponent (Variables|Default|GetRoot) _attachtransform_3 "HandSocket" "KeepWorld" "KeepRelative" "KeepWorld" true)
                  (Transformation|AttachComponentToComponent (Variables|Default|GetPhysicsConstraint) _attachtransform_3 "HandSocket" "KeepWorld" "KeepRelative" "KeepWorld" true)
                  (Transformation|AttachComponentToComponent (Variables|Default|GetMainMesh) (Variables|Default|GetRoot) "None" "KeepWorld" "KeepWorld" "KeepWorld" true)
                  (Variables|/Script/Engine.SceneComponent|SetbAbsoluteLocation (Variables|Default|GetMainMesh) false)
                  (Transformation|SetRelativeLocationAndRotation _mainmesh_4 (.location _inttransform) (.rotation _inttransform) false true) ; Creating a new pivot
                  (Physics|SetSimulatePhysics _mainmesh_4 true)
                  (Class|PhysicsConstraintComponent|SetConstrainedComponents (Variables|Default|GetPhysicsConstraint) (Variables|Default|GetRoot) "None" _mainmesh_4 "None")
                  ;;[1 1 1] Returning from where you got it
                  (Utilities|FlowControl|Delay 0.0)
                  (Transformation|SetWorldLocationAndRotation _mainmesh_4 (.location (Variables|Default|GetBeforeAction)) (.rotation (Variables|Default|GetBeforeAction)) false true)
                  (CallFunction|HitCustom 0 0 0 "0, 0, 0" (Collision|MakeHitResult false false 0.0 0.0 "0, 0, 0" "0, 0, 0" "0,0,1" "0,0,1" 0 0))
                  ;;[1 1 1] Returning collisions
                  (Utilities|FlowControl|RetriggerableDelay 0.1)
                  (if (Variables|Default|GetAttach)
                    (Utilities|DefaultCollision)
                    (Collision|SetCollisionResponsetoChannel (Variables|Default|GetMainMesh) "ECC_Pawn" "ECR_Ignore")))))))
        (:then_1
          (Utilities|FlowControl|Delay 0.0)
          (Class|PrimitiveComponent|WakeAllRigidBodies (Variables|Default|GetMainMesh)))))))

(event Custom|SweepMeshOff
  ;[1 1 1] Hit
  ;;[0 0 0] FixWallPassThrough
  ;;;[1 1 1] Used in child classes. (BP_PickUp_Hard)
)

(event Custom|Free
  ;[1 1 1] Hit
  ;;[1 1 1] Used in child classes. BP_PickUp_Hard
)

(event Custom|Lock
  ;[1 1 1] Hit
  ;;[1 1 1] Used in child classes. BP_PickUp_Hard
)

(event Custom|SweepMeshHit
  (params (HitComponent :type Primitive%20Component%20Object%20Reference) (OtherActor :type Actor%20Object%20Reference) (OtherComp :type Primitive%20Component%20Object%20Reference) (NormalImpulse :type Vector) (Hit :type Hit%20Result%20Structure%20%28by%20ref%29))
  (bind _mainmesh (Variables|Default|GetMainMesh))
  (bind _mainmesh_2 (Variables|Default|GetMainMesh))
  (bind _returnvalue (Transformation|GetWorldLocation _mainmesh))
  ;[1 1 1] Hit
  ;;[0 0 0] FixWallPassThrough
  (if (Variables|Default|GetAttach)
    (Utilities|FlowControl|Delay 0.0)
    (if (> (Math|Vector|Distance(Vector) (Transformation|GetWorldLocation (Variables|Default|GetMainMesh)) (Transformation|GetWorldLocation (Variables|Default|GetSweepMesh))) 2e+01)
      (Utilities|FlowControl|DoOnce false :!label _label
        (:Completed
          (Variables|Default|SetHit Hit)
          (Utilities|FlowControl|Sequence
            (:then_0
              (Variables|Default|SetFixWallPassActive true)
              (Rendering|SetVisibility (Variables|Default|GetSweepMesh) true false)
              (Rendering|SetVisibility _mainmesh_2 false false)
              (Collision|SetCollisionResponsetoAllChannels _mainmesh_2 "ECR_Ignore")
              (Variables|Default|SetTickForSweep false)
              (CallFunction|SweepMeshon))
            (:then_1
              (goto _label_2 Open))
            (:then_2
              (Utilities|FlowControl|Gate true :!label _label_2
                (:Exit
                  (Utilities|FlowControl|Sequence
                    (:then_0
                      (if (and (< (Math|Vector|Distance(Vector) _returnvalue (+ (.ImpactPoint (Collision|BreakHitResult (Variables|Default|GetHit))) (* (.ImpactNormal (Collision|BreakHitResult (Variables|Default|GetHit))) 5.0))) (Math|Vector|Distance(Vector) _returnvalue (.ImpactPoint (Collision|BreakHitResult (Variables|Default|GetHit))))) (> (Math|Vector|Distance(Vector) _returnvalue (.ImpactPoint (Collision|BreakHitResult (Variables|Default|GetHit)))) 25.0)) ; Waiting for MainMesh to return to normal.
                        (Utilities|FlowControl|Sequence
                          (:then_0
                            (Utilities|FlowControl|Sequence
                              (:then_0
                                (goto _label_2 Close))
                              (:then_1
                                (Variables|Default|SetFixWallPassActive false))
                              (:then_2
                                (goto _label Reset))))
                          (:then_1
                            (Rendering|SetVisibility (Variables|Default|GetSweepMesh) false false)
                            (Rendering|SetVisibility (Variables|Default|GetMainMesh) true false)
                            (CallFunction|SweepMeshOff)
                            (if (Variables|Default|GetAttach)
                              (Utilities|DefaultCollision)
                              (Collision|SetCollisionResponsetoChannel (Variables|Default|GetMainMesh) "ECC_Pawn" "ECR_Ignore")
                              (Variables|Default|SetTickForSweep true))))))
                    (:then_1
                      (Utilities|FlowControl|Delay 0.0)
                      (goto _label_2))))))))))))

(event Custom|StopSweep
  (bind _mainmesh (Variables|Default|GetMainMesh))
  (bind _mainmesh_2 (Variables|Default|GetMainMesh))
  (bind _returnvalue (Transformation|GetWorldLocation _mainmesh))
  ;[1 1 1] Hit
  ;;[0 0 0] FixWallPassThrough
  (Transformation|SetWorldTransform (Variables|Default|GetMainMesh) (Transformation|GetWorldTransform (Variables|Default|GetSweepMesh)) false true)
  (Utilities|FlowControl|Sequence
    (:then_0
      (Utilities|FlowControl|Sequence
        (:then_0
          (Utilities|FlowControl|Gate true) ; enters at Close
        )
        (:then_1
          (Variables|Default|SetFixWallPassActive false))
        (:then_2
          (Utilities|FlowControl|DoOnce false) ; enters at Reset
        )))
    (:then_1
      (Rendering|SetVisibility (Variables|Default|GetSweepMesh) false false)
      (Rendering|SetVisibility (Variables|Default|GetMainMesh) true false)
      (CallFunction|SweepMeshOff)
      (if (Variables|Default|GetAttach)
        (Utilities|DefaultCollision)
        (Collision|SetCollisionResponsetoChannel (Variables|Default|GetMainMesh) "ECC_Pawn" "ECR_Ignore")
        (Variables|Default|SetTickForSweep true)))))

(event Custom|SweepMeshOn
  ;[1 1 1] Hit
  ;;[0 0 0] FixWallPassThrough
  ;;;[1 1 1] Used in child classes. (BP_PickUp_Hard)
)

(event EventBeginPlay
  (bind _root (Variables|Default|GetRoot))
  ;[1 1 1] BeginPlay
  (Utilities|IsValid (Variables|Default|GetPhysicsConstraint)
    (:Is%20Valid
      (Utilities|FlowControl|Sequence
        (:then_0
          (Collision|BindEventtoOnComponentHit (Variables|Default|GetMainMesh) (EventDispatchers|CreateEvent :!event Custom|HitCustom))
          (if (Utilities|Enum|Equal(Enum) (Collision|GetCollisionEnabled (Variables|Default|GetMainMesh)) "QueryAndPhysics")
            (Physics|SetSimulatePhysics (Variables|Default|GetMainMesh) (Variables|Tunemeup|GetStartPhysics)))
          (Transformation|SetAbsolute _root false true false)
          (Transformation|SetWorldRotation _root "0, 0, 0" false false))
        (:then_1
          (if (Variables|Tunemeup|GetFixWallPassThrough)
            (Collision|BindEventtoOnComponentHit (Variables|Default|GetSweepMesh) (EventDispatchers|CreateEvent :!event Custom|SweepMeshHit))))))))

(event EventTick
  (params (DeltaSeconds :type Float%20%28single-precision%29))
  ;[1 1 1] EventTick
  ;;[1 1 1] Comment
)

(event EventPickup
  (params (Accurate :type Boolean) (Hit :type Hit%20Result%20Structure) (HideHandIco :type Boolean) (AttachTransform :type SG%20Virtual%20Hand%20Component%20Object%20Reference) (SetAccurate :type Boolean))
  (bind _mainmesh (Variables|Default|GetMainMesh))
  (bind _mainmesh_2 (Variables|Default|GetMainMesh))
  (bind _inttransform (Variables|Default|GetIntTransform))
  (bind _physicsconstraint (Variables|Default|GetPhysicsConstraint))
  (bind _mainmesh_3 (Variables|Default|GetMainMesh))
  (bind _mainmesh_4 (Variables|Default|GetMainMesh))
  ;[1 1 1] Pickup
  (Variables|Default|SetAttachTransform AttachTransform)
  (Utilities|FlowControl|Sequence
    (:then_0
      (if SetAccurate
        (Variables|TuneMeUp|SetAccurate Accurate))
      (Variables|Default|SetHitClick Hit)
      ;;[1 1 1] Adding stability to items
      (if (<= (Variables|Tunemeup|GetSuppressionInertia) 1.0)
        _
        (else
          (Class|PhysicsConstraintComponent|SetAngularDriveMode _physicsconstraint (select (Variables|TuneMeUp|GetAccurate) "SLERP" "TwistAndSwing"))
          (Class|PhysicsConstraintComponent|SetAngularVelocityDriveTwistandSwing _physicsconstraint (not (Variables|TuneMeUp|GetAccurate)) (not (Variables|TuneMeUp|GetAccurate)))
          (Class|PhysicsConstraintComponent|SetOrientationDriveTwistandSwing _physicsconstraint (not (Variables|TuneMeUp|GetAccurate)) (not (Variables|TuneMeUp|GetAccurate)))
          (Class|PhysicsConstraintComponent|SetAngularDriveParams _physicsconstraint 5e+01 (Math|Float|SelectFloat 1.0 (Variables|Tunemeup|GetSuppressionInertia) (Variables|TuneMeUp|GetAccurate)) 0.0)))
      (Variables|Default|SetAttach true)
      (Input|EnableInput (Game|GetPlayerController 0))
      (Utilities|IsValid (Variables|Default|GetPhysicsConstraint)
        (:Is%20Valid
          ;;[1 1 1] For stability.
          (if (or (Physics|IsSimulatingPhysics _mainmesh "None") (Variables|Default|GetRotate))
            _
            (else
              (Utilities|FlowControl|Delay 0.0)
              (Physics|SetSimulatePhysics _mainmesh true)))
          (Utilities|FlowControl|Sequence
            (:then_0
              (Class|PhysicsConstraintComponent|BreakConstraint (Variables|Default|GetPhysicsConstraint))
              ;;[1 1 1] Memorise the default collision
              (Utilities|Array|Clear (Variables|Default|GetIntCollision))
              (bind _enumvalue (|ForEachECollisionChannel)
                (:LoopBody
                  (Utilities|Array|Add (Variables|Default|GetIntCollision) (Collision|GetCollisionResponsetoChannel (Variables|Default|GetMainMesh) _enumvalue)))
                (:then
                  (Collision|SetCollisionResponsetoChannel (Variables|Default|GetMainMesh) "ECC_Pawn" "ECR_Ignore")
                  (Variables|Default|SetBeforeAction (Transformation|GetWorldTransform (Variables|Default|GetMainMesh)))
                  (Variables|/Script/Engine.SceneComponent|SetbAbsoluteLocation (Variables|Default|GetMainMesh) true)
                  (Variables|/Script/Engine.SceneComponent|SetbAbsoluteLocation (Variables|Default|GetPhysicsConstraint) true)
                  (if (Variables|Tunemeup|GetFixWallPassThrough)
                    (Variables|Default|SetTickForSweep true)
                    (Rendering|SetVisibility (Variables|Default|GetSweepMesh) false false))
                  (if (Variables|TuneMeUp|GetAccurate)
                    ;;[0 0 0] Accurate
                    (if (Variables|Default|GetRotate)
                      (Transformation|SetWorldLocationAndRotation _mainmesh_3 (.location (Variables|Default|GetLast)) (.rotation (Variables|Default|GetLast)) false true)
                      (Collision|SetCollisionResponsetoAllChannels _mainmesh_3 "ECR_Overlap") ; To prevent nearby meshes from flying off
                    )
                    (Transformation|SetWorldLocation (Variables|Default|GetRoot) (.ImpactPoint (Collision|BreakHitResult (Variables|Default|GetHitClick))) false true)
                    (Physics|SetSimulatePhysics _mainmesh_2 true)
                    (Class|PhysicsConstraintComponent|SetConstrainedComponents (Variables|Default|GetPhysicsConstraint) (Variables|Default|GetRoot) "None" _mainmesh_2 "None")
                    (if (Variables|Default|GetRotate)
                      ;;;[1 1 1] Solves a lot of problems when returning from inspection
                      (Transformation|SetWorldLocation (Variables|Default|GetPhysicsConstraint) (+ (Transformation|GetWorldLocation (Variables|Default|GetAttachTransform)) (* (Math|Vector|GetForwardVector (Variables|Default|GetAttachTransform)) (Math|Vector|Distance(Vector) (Transformation|GetWorldLocation (Variables|Default|GetAttachTransform)) (.location (Variables|Default|GetBeforeAction))))) false true)
                      (else
                        (Transformation|AttachComponentToComponent (Variables|Default|GetRoot) (Variables|Default|GetAttachTransform) "HandSocket" "KeepWorld" "KeepWorld" "KeepWorld" true)
                        (Transformation|AttachComponentToComponent (Variables|Default|GetPhysicsConstraint) (Variables|Default|GetAttachTransform) "HandSocket" "KeepWorld" "KeepWorld" "KeepWorld" true)))
                    (Utilities|FlowControl|Sequence
                      (:then_0
                        (if (Variables|Default|GetRotate)
                          ;;;[1 1 1] Returning from where you got it
                          (Utilities|FlowControl|Delay 0.0)
                          (Transformation|SetWorldLocationAndRotation (Variables|Default|GetMainMesh) (.location (Variables|Default|GetBeforeAction)) (.rotation (Variables|Default|GetBeforeAction)) false true)
                          (Utilities|DefaultCollision)
                          (Collision|SetCollisionResponsetoChannel (Variables|Default|GetMainMesh) "ECC_Pawn" "ECR_Ignore")
                          (else
                            (Variables|Default|SetLast (Transformation|GetWorldTransform (Variables|Default|GetMainMesh)))))))
                    (else
                      ;;[1 1 1] Ignore other physical subjects.
                      (if (Variables|Tunemeup|GetIgnoreCamera?)
                        _
                        (else
                          (Collision|SetCollisionResponsetoChannel (Variables|Default|GetMainMesh) "ECC_PhysicsBody" "ECR_Ignore")))
                      (Transformation|SetWorldLocation (Variables|Default|GetRoot) (.ImpactPoint (Collision|BreakHitResult (Variables|Default|GetHitClick))) false true)
                      (Transformation|AttachComponentToComponent (Variables|Default|GetRoot) (Variables|Default|GetAttachTransform) "HandSocket" "KeepWorld" "KeepRelative" "KeepWorld" true)
                      (Transformation|AttachComponentToComponent (Variables|Default|GetPhysicsConstraint) (Variables|Default|GetAttachTransform) "HandSocket" "KeepWorld" "KeepRelative" "KeepWorld" true)
                      (Transformation|AttachComponentToComponent (Variables|Default|GetMainMesh) (Variables|Default|GetRoot) "None" "KeepWorld" "KeepWorld" "KeepWorld" true)
                      (Variables|/Script/Engine.SceneComponent|SetbAbsoluteLocation (Variables|Default|GetMainMesh) false)
                      (Transformation|SetRelativeLocationAndRotation _mainmesh_4 (.location _inttransform) (.rotation _inttransform) false true) ; Creating a new pivot
                      (Physics|SetSimulatePhysics _mainmesh_4 true)
                      (Class|PhysicsConstraintComponent|SetConstrainedComponents (Variables|Default|GetPhysicsConstraint) (Variables|Default|GetRoot) "None" _mainmesh_4 "None")
                      ;;[1 1 1] Returning from where you got it
                      (Utilities|FlowControl|Delay 0.0)
                      (Transformation|SetWorldLocationAndRotation _mainmesh_4 (.location (Variables|Default|GetBeforeAction)) (.rotation (Variables|Default|GetBeforeAction)) false true)
                      (CallFunction|HitCustom 0 0 0 "0, 0, 0" (Collision|MakeHitResult false false 0.0 0.0 "0, 0, 0" "0, 0, 0" "0,0,1" "0,0,1" 0 0))
                      ;;[1 1 1] Returning collisions
                      (Utilities|FlowControl|RetriggerableDelay 0.1)
                      (if (Variables|Default|GetAttach)
                        (Utilities|DefaultCollision)
                        (Collision|SetCollisionResponsetoChannel (Variables|Default|GetMainMesh) "ECC_Pawn" "ECR_Ignore")))))))
            (:then_1
              (Utilities|FlowControl|Delay 0.0)
              (Class|PrimitiveComponent|WakeAllRigidBodies (Variables|Default|GetMainMesh)))))))
    (:then_1
      (Default|CallEDPickup))))

(event EventDrop
  (params (Throw? :type Boolean))
  ;[1 1 1] Drop
  (Utilities|FlowControl|Sequence
    (:then_0
      (if (Variables|Tunemeup|GetFixWallPassThrough)
        (CallFunction|StopSweep))
      (Variables|Default|SetAttach false)
      (Class|PhysicsConstraintComponent|BreakConstraint (Variables|Default|GetPhysicsConstraint))
      (Utilities|FlowControl|Sequence
        (:then_0
          (Utilities|DefaultCollision)
          (Utilities|Array|Clear (Variables|Default|GetIntCollision))
          (Input|DisableInput (Game|GetPlayerController 0)))
        (:then_1
          (Utilities|FlowControl|Delay 0.0)
          (Class|PrimitiveComponent|WakeAllRigidBodies (Variables|Default|GetMainMesh)))
        (:then_2
          (Utilities|FlowControl|RetriggerableDelay 1.0)
          (if (not (Variables|Default|GetAttach))
            (Variables|Default|SetTickForSweep false)
            (Transformation|DetachFromComponent (Variables|Default|GetRoot) "KeepWorld" "KeepRelative" "KeepWorld" true)))
        (:then_3
          (Variables|Default|SetAttachTransform 0))))
    (:then_1
      (Default|CallEDDrop)
      (Utilities|IsValid (Variables|Default|GetAttachTransform)
        (:Is%20Valid
          (Physics|SetPhysicsLinearVelocity (Variables|Default|GetMainMesh) (Math|Vector|SelectVector (* (Transformation|GetWorldLocation (Variables|Default|GetAttachTransform)) (* 5e+03 (Variables|Tunemeup|GetSpeedAfterDrop))) (* (Transformation|GetComponentVelocity (Variables|Default|GetMainMesh)) (Variables|Tunemeup|GetSpeedAfterDrop)) Throw?) false "None"))))))

(fn ConstructionScript
  (bind _mainmesh (Variables|Default|GetMainMesh))
  (Variables|Default|SetIntTransform (Transformation|GetRelativeTransform (Variables|Default|GetMainMesh)))
  ;[1 1 1] Creating a mesh to be moved via "Sweep"
  (if (Variables|Tunemeup|GetFixWallPassThrough)
    (bind _returnvalue (AddComponent|AddStaticMeshComponent true))
    (bind _output_get (Variables|Default|SetSweepMesh _returnvalue))
    (Transformation|SetAbsolute _output_get true true true)
    (Collision|SetCollisionResponsetoChannel (Variables|Default|GetSweepMesh) "ECC_PhysicsBody" "ECR_Ignore")
    (Collision|SetCollisionResponsetoChannel (Variables|Default|GetSweepMesh) "ECC_Pawn" "ECR_Ignore")
    (Rendering|SetVisibility (Variables|Default|GetSweepMesh) false false)
    (Components|StaticMesh|SetStaticMesh (Variables|Default|GetSweepMesh) (Variables|/Script/Engine.StaticMeshComponent|GetStaticMesh _mainmesh))
    (Collision|SetCollisionEnabled (Variables|Default|GetSweepMesh) "QueryOnly")
    (Transformation|SetWorldTransform (Variables|Default|GetSweepMesh) (Transformation|GetWorldTransform _mainmesh) false true)
    (for (_array_element _array_index) (Rendering|Material|GetMaterials _mainmesh)
      (Rendering|Material|SetMaterial (Variables|Default|GetSweepMesh) _array_index _array_element))))

(fn AttachLocation
  (bind _returnvalue (Game|GetPlayerCameraManager 0))
  (bind _offset (Variables|Tunemeup|GetOffset))
  (bind _transformcomponent (Variables|/Script/Engine.PlayerCameraManager|GetTransformComponent _returnvalue))
  (bind _returnvalue_2 (Transformation|GetWorldLocation _transformcomponent))
  (bind _returnvalue_3 (Math|Vector|GetForwardVector _transformcomponent))
  (return (+ _returnvalue_2 (* _returnvalue_3 (Math|Float|SelectFloat (Math|Vector|Distance(Vector) (- (Transformation|GetWorldLocation (Variables|Default|GetMainMesh)) (.Location (Math|Transform|BreakTransform (Variables|Default|GetIntTransform)))) _returnvalue_2) 2.5e+02 false)) (+ (* _returnvalue_3 (.x _offset)) (* (Math|Vector|GetRightVector _transformcomponent) (.y _offset)) (* (Math|Vector|GetUpVector _transformcomponent) (.z _offset))))))