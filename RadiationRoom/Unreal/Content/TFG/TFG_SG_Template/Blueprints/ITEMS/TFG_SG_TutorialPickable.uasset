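; Tutorial pickable item that reports when the player detects or grabs it, via detection and interaction dispatcher calls gated by flags.
; A Spawn event plays a cartoon pop, then after a short delay reveals the item, enables physics and makes it interactable.
; A Liar flag turns it into a decoy: it overrides the grab type, shows its widget on detection and never reports a grab.
; Cancelling interaction re-enables physics.
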(event Custom|Spawn
  (Audio|PlaySoundatLocation "/Game/Game/Assets/Sounds/effects/cartoon_pop.cartoon_pop" (Transformation|GetWorldLocation (Variables|Default|GetStaticMesh)) "0, 0, 0" 1.0 1.0 0.0 0 0 0 0)
  (Utilities|FlowControl|Delay 0.2)
  (Rendering|SetActorHiddenInGame false)
  (Physics|SetSimulatePhysics (Variables|Default|GetStaticMesh) true)
  (Variables|Default|SetCanBeInteracted true))

(event Custom|CancelInteract_1
  (params (Player :type Pawn%20Object%20Reference))
  (Physics|SetSimulatePhysics (Variables|Default|GetStaticMesh) true))

(event Custom|StopDetection_1
  (params (Player :type BP%20Player%20Object%20Reference)))

(event Custom|StartDetection_1
  (params (Player :type BP%20Player%20Object%20Reference))
  (if (Variables|Default|GetCanBeDetected)
    (Variables|Default|SetHasBeenDetected true)
    (Default|CallEDDetectionStarted)
    (if (Variables|Default|GetLiar)
      (Development|SetHiddeninGame (Variables|Default|GetWidget) false false))))

(event Custom|InteractWith_1
  (params (Player :type Pawn%20Object%20Reference))
  (if (and (not (Variables|Default|GetLiar)) (Variables|Default|GetCanBeGrabbed))
    (Variables|Default|SetHasBeenGrabbed true)
    (Default|CallEDInteractionStarted)))

(event EventBeginPlay
  (|CallParentFunction)
  (if (Variables|Default|GetLiar)
    (Variables|/Game/VRTemplate/Blueprints/GrabComponent.GrabComponent_C|SetGrabType (Variables|Default|GetGrabComponent) "NewEnumerator0")))

(fn ConstructionScript)