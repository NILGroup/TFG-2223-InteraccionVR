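; Pickable EPD dosimeter Blueprint that, as wired, adds no working behavior of its own and only forwards BeginPlay, Tick and construction to its parent.
; A disconnected chain would push ACRadiation dose rate and absorption to an info widget, send a database event, then call ShowRadiation after a short delay.
; SetEPDId is an unfinished stub that gathers BP_Dosimeter_EPD actors and tests for an empty list without assigning an ID.
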(event EventBeginPlay
  (|CallParentFunction))

(event EventTick
  (params (DeltaSeconds :type Float%20%28single-precision%29))
  (|CallParentFunction DeltaSeconds))

(fn ConstructionScript
  (|CallParentFunction))

(fn SetEPDId
  (bind _outactors (Actor|GetAllActorsOfClass "/Game/Game/Blueprints/Actors/Dosimeters/BP_Dosimeter_EPD.BP_Dosimeter_EPD_C"))
  (if (Utilities|Array|IsEmpty _outactors)
    _))