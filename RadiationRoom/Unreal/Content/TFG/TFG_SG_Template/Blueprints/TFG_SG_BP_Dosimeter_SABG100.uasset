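; SABG100 dosimeter item that measures dose and absorption rates from actors carrying an AC_Radiation component.
; A box overlap starts a self-repeating half-second loop that updates the widget display, which is zeroed shortly after overlap ends.
; Interactable items and NPCs trigger event dispatchers on each reading.
; Their readings are also logged through the game instance's DatabaseManager, provided a BP_RadiationEmissionPoint exists in the level.
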(event OnComponentBeginOverlap(Box)
  (params (OverlappedComponent :type Primitive%20Component%20Object%20Reference) (OtherActor :type Actor%20Object%20Reference) (OtherComp :type Primitive%20Component%20Object%20Reference) (OtherBodyIndex :type Integer) (bFromSweep :type Boolean) (SweepResult :type Hit%20Result%20Structure%20%28by%20ref%29))
  (Utilities|IsValid (Actor|GetComponentbyClass OtherActor "/Game/Game/Blueprints/Components/AC_Radiation.AC_Radiation_C")
    (:Is%20Valid
      (Variables|Default|SetHittingActor OtherActor)
      (Variables|Default|SetMeasuringRadiation true)
      (CallFunction|MeasureRadiation))))

(event OnComponentEndOverlap(Box)
  (params (OverlappedComponent :type Primitive%20Component%20Object%20Reference) (OtherActor :type Actor%20Object%20Reference) (OtherComp :type Primitive%20Component%20Object%20Reference) (OtherBodyIndex :type Integer))
  (if (== OtherActor (Variables|Default|GetHittingActor))
    (Variables|Default|SetMeasuringRadiation false)
    (Variables|Default|SetHittingActor 0)
    (Utilities|FlowControl|Delay 1.0)
    (Default|SetRadiationRate (Variables|Default|GetRadiationInfoWidgetActor) 0.0 0.0)))

(event Custom|MeasureRadiation
  (bind _hittingactor (Variables|Default|GetHittingActor))
  (bind _hittingactor_2 (Variables|Default|GetHittingActor))
  (bind _returnvalue (Actor|GetComponentbyClass _hittingactor "/Game/Game/Blueprints/Components/AC_Radiation.AC_Radiation_C"))
  (bind _doseabsorption (Variables|/Game/Game/Blueprints/Components/AC_Radiation.AC_Radiation_C|GetDoseAbsorption _returnvalue))
  (bind _doserate (Variables|/Game/Game/Blueprints/Components/AC_Radiation.AC_Radiation_C|GetDoseRate _returnvalue))
  (if (Variables|Default|GetMeasuringRadiation)
    (Default|SetRadiationRate (Variables|Default|GetRadiationInfoWidgetActor) _doserate _doseabsorption)
    (bind _asbp_interact_item_parent (Utilities|Casting|CastToBP_InteractItemParent _hittingactor_2)
      (:then
        (Default|CallEDItemRadiationMeasured _asbp_interact_item_parent)
        (CallFunction|SendItemRadiationEventtoDB _asbp_interact_item_parent _doserate _doseabsorption))
      (:CastFailed
        (bind _asbp_npc (Utilities|Casting|CastToBP_NPC _hittingactor_2)
          (:then
            (Default|CallEDNPCRadiationMeasured _asbp_npc)
            (CallFunction|SendNPCRadiationEventtoDB _asbp_npc _doserate _doseabsorption))
          (:CastFailed
            _))))
    (Utilities|FlowControl|Delay 0.5)
    (CallFunction|MeasureRadiation)))

(event EventBeginPlay
  ;[1 1 1] check
  (|CallParentFunction)
  (Utilities|FlowControl|Sequence
    (:then_0
      (bind _aswbp_dosimeter_for_dose_and_absortion_radiation_rate (Utilities|Casting|CastToWBP_DosimeterForDoseAndAbsortionRadiationRate (UserInterface|GetWidget (Variables|Default|GetRadiationInfoWidgetComponent))))
      (Variables|Default|SetRadiationInfoWidgetActor _aswbp_dosimeter_for_dose_and_absortion_radiation_rate))))

(event EventTick
  (params (DeltaSeconds :type Float%20%28single-precision%29))
  (|CallParentFunction DeltaSeconds)
  (if (Variables|Default|GetMeasuringRadiation)
    (Utilities|FlowControl|Delay 0.5)))

(event Custom|SendNPCRadiationEventToDB
  (params (Actor :type BP%20NPC%20Object%20Reference) (Dose%20Rate :type Float%20%28double-precision%29) (DoseAbsortion :type Float%20%28double-precision%29))
  ;[1 1 1] check
  (bind _returnvalue (Actor|GetActorOfClass "/Game/Game/Blueprints/Actors/Radiation/BP_RadiationEmissionPoint.BP_RadiationEmissionPoint_C"))
  (Utilities|IsValid _returnvalue
    (:Is%20Valid
      (bind _asrr_game_instance (Utilities|Casting|CastToRR_GameInstance (Variables|Default|GetGameInstance)))
      (bind _data (Default|GetDataBaseMainInfoEvent _asrr_game_instance))
      (Default|SendNPCRadiationEventtoDB (Variables|/Game/Game/Blueprints/RR_GameInstance.RR_GameInstance_C|GetDatabase%20Manager _asrr_game_instance) (Utilities|Struct|MakeF_NPCRadiationEvent 0 (.user_id (Utilities|Struct|BreakF_MainInfoEvent _data)) (.scenario_type (Utilities|Struct|BreakF_MainInfoEvent _data)) (Variables|/Game/Game/Blueprints/Characters/AI/BP_NPC.BP_NPC_C|GetActorId Actor) Dose%20Rate DoseAbsortion (Math|DateTime|Now))))))

(event Custom|SendItemRadiationEventToDB
  (params (Actor :type BP%20Interact%20Item%20Parent%20Object%20Reference) (Dose%20Rate :type Float%20%28double-precision%29) (DoseAbsortion :type Float%20%28double-precision%29))
  ;[1 1 1] check
  (bind _returnvalue (Actor|GetActorOfClass "/Game/Game/Blueprints/Actors/Radiation/BP_RadiationEmissionPoint.BP_RadiationEmissionPoint_C"))
  (Utilities|IsValid _returnvalue
    (:Is%20Valid
      (bind _asrr_game_instance (Utilities|Casting|CastToRR_GameInstance (Variables|Default|GetGameInstance)))
      (bind _data (Default|GetDataBaseMainInfoEvent _asrr_game_instance))
      (Default|SendItemRadiationEventtoDB (Variables|/Game/Game/Blueprints/RR_GameInstance.RR_GameInstance_C|GetDatabase%20Manager _asrr_game_instance) (Utilities|Struct|MakeF_ItemRadiationEvent 0 (.user_id (Utilities|Struct|BreakF_MainInfoEvent _data)) (.scenario_type (Utilities|Struct|BreakF_MainInfoEvent _data)) (Variables|/Game/Game/Blueprints/Actors/Items/BP_InteractItemParent.BP_InteractItemParent_C|GetActorId Actor) Dose%20Rate DoseAbsortion (Math|DateTime|Now))))))

(fn ConstructionScript
  (|CallParentFunction))

(fn CanUsewith
  (params (Use%20Point :type Actor%20Object%20Reference))
  (return (== (Utilities|GetClass Use%20Point) 0)))