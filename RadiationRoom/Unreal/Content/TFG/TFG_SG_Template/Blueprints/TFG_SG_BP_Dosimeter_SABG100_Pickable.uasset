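; Pickable SABG100 dosimeter Blueprint with a widget component for displaying radiation dose and absorption rates.
; BeginPlay calls the parent and caches the dosimeter widget from RadiationInfoWidgetComponent.
; Measurement logic is disconnected: unwired nodes would update the widget, raise item or NPC measured events, send readings to a database and repeat.
; Tick calls the parent, then only runs a delay with nothing after it.
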(event EventBeginPlay
  ;[1 1 1] check
  (|CallParentFunction)
  (Utilities|FlowControl|Sequence
    (:then_0
      (bind _aswbp_dosimeter_for_dose_and_absortion_radiation_rate (Utilities|Casting|CastToWBP_DosimeterForDoseAndAbsortionRadiationRate (UserInterface|GetWidget (Variables|Default|GetRadiationInfoWidgetComponent))))
      (Variables|Default|SetRadiationInfoWidgetActor _aswbp_dosimeter_for_dose_and_absortion_radiation_rate))))

(event EventTick
  (params (DeltaSeconds :type Float%20%28single-precision%29))
  (|CallParentFunction DeltaSeconds)
  (if true
    (Utilities|FlowControl|Delay 0.5)))

(fn ConstructionScript
  (|CallParentFunction))